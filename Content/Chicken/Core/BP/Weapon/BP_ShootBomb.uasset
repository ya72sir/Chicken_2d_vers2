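; BP_ShootBomb is a trap that fires a bomb along a spline when a player overlaps its box while enabled.
; A bomb with configurable scale and damage waits at the first spline point, spawned at BeginPlay.
; A timeline, sped by setting the actor's CustomTimeDilation to Speed, moves it linearly between the first two spline points, then detonates it.
; A replacement spawns after a short delay, and a flag blocks retriggering meanwhile.
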(event OnComponentBeginOverlap(Box)
  (params (OverlappedComponent :type Primitive%20Component%20Object%20Reference) (OtherActor :type Actor%20Object%20Reference) (OtherComp :type Primitive%20Component%20Object%20Reference) (OtherBodyIndex :type Integer) (bFromSweep :type Boolean) (SweepResult :type Hit%20Result%20Structure%20%28by%20ref%29))
  (bind _spline (Variables|Default|GetSpline))
  (if (Variables|Default|GetEnabled?)
    (bind _isplayer_ (Class|BPIPlayer|BPIIsPlayer?(Message) OtherActor))
    (if _isplayer_
      (if (not (Variables|Default|GetisBombMove?))
        (Variables|/Script/Engine.Actor|SetCustomTimeDilation self (Variables|Default|GetSpeed))
        (Variables|Default|SetisBombMove? true)
        (bind _newtrack_0 (Timeline|SetLocation PlayFromStart)
          (:Update
            (bind _bp_activebomb (Variables|Default|GetBP_ActiveBomb)
              (:then
                (Transformation|SetActorLocation _bp_activebomb (Math|Vector|Lerp(Vector) (Spline|GetLocationatSplinePoint _spline 0 "World") (Spline|GetLocationatSplinePoint _spline 1 "World") _newtrack_0) false false))
              (:else)))
          (:Finished
            (bind _bp_activebomb_2 (Variables|Default|GetBP_ActiveBomb)
              (:then
                (Default|EvBombExplosion _bp_activebomb_2))
              (:else
                _))
            (Utilities|FlowControl|Delay 2.0)
            (CallFunction|FSpawnBomb)
            (Variables|Default|SetisBombMove? false)))))))

(event EventBeginPlay
  (CallFunction|FSpawnBomb))

(fn ConstructionScript)

(fn FSpawnBomb
  (bind _spline (Variables|Default|GetSpline))
  (bind _returnvalue (Spline|GetTransformatSplinePoint _spline 0 "World" false))
  (bind _returnvalue_2 (Game|SpawnActorfromClass "/Game/Chicken/Core/BP/Weapon/BP_Bomb.BP_Bomb_C" (Math|Transform|MakeTransform (.location _returnvalue) (.rotation _returnvalue) (Variables|Default|GetScaleBomb)) "AlwaysSpawn" 0 (Variables|Default|GetDamage) 0))
  (Variables|Default|SetBP_ActiveBomb _returnvalue_2))