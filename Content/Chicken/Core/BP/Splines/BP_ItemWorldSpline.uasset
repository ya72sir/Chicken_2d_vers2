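; BP_ItemWorldSpline lays out a row of world items, such as damage or bitcoin pickups, along a spline.
; Its construction script builds a straight or three-point curved spline, then spawns scaled child actors of the chosen class at fixed distance intervals.
; Damage and bitcoin children receive this actor as parent.
; A shared audio component plays sounds through FPlaySound, either looping with a short delay or clearing its active flag when finished.
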(event OnAudioFinished(Audio)
  (Utilities|FlowControl|Delay 0.5)
  (if (Variables|Default|GetLoopSound?)
    (bind _audio (Variables|Default|GetAudio)
      (:then
        (Audio|Components|Audio|Play _audio 0.0))
      (:else))
    (else
      (Variables|Default|SetSettingsForSoundActive? false))))

(fn ConstructionScript
  (Spline|ClearSplinePoints (Variables|Default|GetSpline) true)
  (if (Variables|Default|GetuseCurve?)
    (Class|SplineComponent|AddPoints (Variables|Default|GetSpline) (Utilities|Array|MakeArray (Utilities|Struct|MakeSplinePoint 0.0 (Variables|Default|Getpoint01)) (Utilities|Struct|MakeSplinePoint 1.0 (Variables|Default|GetpointMiddle)) (Utilities|Struct|MakeSplinePoint 2.0 (Variables|Default|Getpoint02))) true)
    (else
      (Class|SplineComponent|AddPoints (Variables|Default|GetSpline) (Utilities|Array|MakeArray (Utilities|Struct|MakeSplinePoint 0.0 (Variables|Default|Getpoint01)) (Utilities|Struct|MakeSplinePoint 1.0 (Variables|Default|Getpoint02))) true)))
  (for _index (range 0 (.ReturnValue (Math|Float|Division(WholeandRemainder) (Spline|GetSplineLength (Variables|Default|GetSpline)) (Variables|Default|GetDivisor))))
    (bind _returnvalue (AddComponent|AddChildActorComponent false (Math|Transform|MakeTransform (Spline|GetLocationatDistanceAlongSpline (Variables|Default|GetSpline) (* _index (Variables|Default|GetDivisor)) "Local") "0, 0, 0" "0.200000,0.200000,0.200000")))
    (ChildActorComponent|SetChildActorClass _returnvalue (Variables|Default|GetItemWorld))
    (Transformation|SetWorldScale3D _returnvalue (Variables|Default|GetWorldScale3d))
    (bind _asbp_damage (Utilities|Casting|CastToBP_Damage (Variables|/Script/Engine.ChildActorComponent|GetChildActor _returnvalue))
      (:then
        (Variables|/Game/Chicken/Core/BP/ActorsForLevel/BP_Damage.BP_Damage_C|SetActorParent _asbp_damage self))
      (:CastFailed
        (bind _asbp_money_bitcoin (Utilities|Casting|CastToBP_MoneyBitcoin (Variables|/Script/Engine.ChildActorComponent|GetChildActor _returnvalue)))
        (Variables|/Game/Chicken/Core/BP/BP_MasterForSpline/ActorsForSpline/BP_MoneyBitcoin.BP_MoneyBitcoin_C|SetActorParent _asbp_money_bitcoin self)))))

(fn FPlaySound
  (params (Loop? :type Boolean) (Sound :type Sound%20Base%20Object%20Reference))
  (bind _audio (Variables|Default|GetAudio))
  (Variables|Default|SetLoopSound? Loop?)
  (Variables|Default|SetSettingsForSoundActive? true)
  (Variables|/Script/Engine.AudioComponent|SetSound _audio Sound)
  (Audio|Components|Audio|Stop _audio)
  (Audio|Components|Audio|Play _audio 0.0))