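; BP_Weapon_Damage is a one-shot damage actor among the spline actors, with a sphere trigger, Paper2D sprite and particle system.
; On sphere overlap, it sends a character damage interface message to the other actor and proceeds only if that returns true.
; It then applies fixed point damage, disables collision, hides the sprite, activates the particles and destroys itself after a short delay.
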(event OnComponentBeginOverlap(Sphere)
  (params (OverlappedComponent :type Primitive%20Component%20Object%20Reference) (OtherActor :type Actor%20Object%20Reference) (OtherComp :type Primitive%20Component%20Object%20Reference) (OtherBodyIndex :type Integer) (bFromSweep :type Boolean) (SweepResult :type Hit%20Result%20Structure%20%28by%20ref%29))
  (bind _damageisenabled_ (Class|BPICharacter|BPICharacterDamage(Message) OtherActor))
  (if _damageisenabled_
    (Game|Damage|ApplyPointDamage OtherActor 1e+01 (Math|Vector|MakeVector 3.0 3.0 3.0) (Collision|MakeHitResult false false 0.0 0.0 "0, 0, 0" "0, 0, 0" "0,0,1" "0,0,1" 0 0))
    (Collision|SetActorEnableCollision false)
    (Rendering|SetVisibility (Variables|Default|GetPaperSprite) false false)
    (Components|Activation|SetActive (Variables|Default|GetParticleSystem) true true)
    (Utilities|FlowControl|Delay 1.0)
    (Actor|DestroyActor)))

(fn ConstructionScript)