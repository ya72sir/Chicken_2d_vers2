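; Master spline-based world item that carries a moving actor, spawns actors along its path and can act as a water zone.
; Construction, rerun on BeginPlay, loads an enum-selected DataTable preset, builds the spline and places child actors at intervals.
; While active, Tick moves a child actor along the spline, reversing or destroying and respawning it at the end.
; Activation also applies particle, sound and sprite; spline mesh overlaps track the player, and interface calls activate by ID.
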(event OnAudioFinished(Audio)
  (if (Variables|Param/Audio|GetSoundIsRepeat?)
    (Audio|Components|Audio|Play (Variables|Default|GetAudio) 0.0)))

(event EventTick
  (params (DeltaSeconds :type Float%20%28single-precision%29))
  (if (Variables|Param|GetActive?)
    (Variables|Private|SetDelta (* DeltaSeconds (Variables|Param/Move|GetSpeed_Move)))
    (CallFunction|EvMove DeltaSeconds)
    (Utilities|MMoveSetRotation)))

(event EventBPIActivateActor
  (params (ID :type Integer))
  (if (== ID (Variables|Param|GetId))
    (CallFunction|EvActive true)))

(fn ConstructionScript
  (CallFunction|FConstruction))

(fn FConstruction
  (bind _returnvalue (Transformation|GetActorLocation))
  (bind _arrchildactor (Variables|Default|GetarrChildActor))
  (bind (_x _y _z) (Math|Vector|BreakVector _returnvalue))
  (|WriteID_2
    (:Completed
      (for _array_element _arrchildactor
        (Components|DestroyComponent _array_element))
      (Utilities|Array|Clear _arrchildactor)
      (Transformation|SetActorLocation (Math|Vector|MakeVector _x (Variables|Default|GetLayerInWorld) _z) false false)
      (if (Utilities|Enum|NotEqual(Enum) (Utilities|String|EnumtoString (Variables|Param|GetEExampleWorldItems)) "None")
        (Utilities|MGetDataTable
          (:RowNotFound
            _)
          (:then
            _)))
      (Utilities|MBuildSpline)
      (Utilities|FlowControl|Sequence
        (:then_0
          (CallFunction|EvActive (Variables|Param|GetActive?)))
        (:then_1
          (if (Variables|Param|GetActive?)
            (Variables|Param/SpawnsActorsAlongSpline|GetActor%20for%20spawn%20along%20spline
              (:then
                (for _index (range 0 (.ReturnValue (Math|Float|Division(WholeandRemainder) (Spline|GetSplineLength (Variables|Default|GetSpline)) (Variables|Param/SpawnsActorsAlongSpline|GetDivider%20for%20the%20actor%20along%20the%20spline))))
                  (bind _returnvalue_2 (AddComponent|AddChildActorComponent false (Math|Transform|MakeTransform (Spline|GetLocationatDistanceAlongSpline (Variables|Default|GetSpline) (* _index (Variables|Param/SpawnsActorsAlongSpline|GetDivider%20for%20the%20actor%20along%20the%20spline)) "Local") "0, 0, 0" (Variables|Param/SpawnsActorsAlongSpline|GetWorld%20Scale%203d%20For%20Spawns%20Actors%20Along%20Spline))))
                  (ChildActorComponent|SetChildActorClass _returnvalue_2 (Variables|Param/SpawnsActorsAlongSpline|GetActor%20for%20spawn%20along%20spline))
                  (Utilities|Array|Add (Variables|Default|GetarrChildActor) _returnvalue_2)))
              (:else))))))))

(fn BPIGetActorID
  (return (Variables|Param|GetId)))

(fn BPIOpenDoor
  (return false))

(event OnComponentBeginOverlap(SplineMesh)
  (params (OverlappedComponent :type Primitive%20Component%20Object%20Reference) (OtherActor :type Actor%20Object%20Reference) (OtherComp :type Primitive%20Component%20Object%20Reference) (OtherBodyIndex :type Integer) (bFromSweep :type Boolean) (SweepResult :type Hit%20Result%20Structure%20%28by%20ref%29))
  (if (Variables|Param|GetActive?)
    (bind (_isplayer_ _player) (Class|BPIPlayer|BPIIsPlayer?(Message) OtherActor))
    (if _isplayer_
      (bind _output_get (Variables|Private|SetPlayer _player))
      (CallFunction|EvOverlapBegin)
      (if (Variables|Param/Additional|GetSetIsWater?)
        (Variables|/Game/Chicken/Core/BP_Characters/BP_Player/Level/BP_Player2D.BP_Player2D_C|SetbWater? _output_get true)))))

(event OnComponentEndOverlap(SplineMesh)
  (params (OverlappedComponent :type Primitive%20Component%20Object%20Reference) (OtherActor :type Actor%20Object%20Reference) (OtherComp :type Primitive%20Component%20Object%20Reference) (OtherBodyIndex :type Integer))
  (bind _isplayer_ (Class|BPIPlayer|BPIIsPlayer?(Message) OtherActor))
  (if _isplayer_
    (CallFunction|EvOverlapEnd)
    (if (Variables|Param/Additional|GetSetIsWater?)
      (bind _player (Variables|Private|GetPlayer)
        (:then
          (Variables|/Game/Chicken/Core/BP_Characters/BP_Player/Level/BP_Player2D.BP_Player2D_C|SetbWater? _player false))
        (:else
          _)))
    (Variables|Private|SetPlayer 0)))

(event Custom|EvOverlapBegin)

(event Custom|EvOverlapEnd)

(event Custom|EvMove
  (params (Tick :type Float%20%28single-precision%29))
  (if (Variables|Param|GetActive?)
    (if (Variables|Param/Move|GetActorIsMove?)
      (Variables|Param/Move|GetActorForMove
        (:then
          (bind _actorcomponent (Variables|Default|GetActorComponent)
            (:then
              (Variables|/Script/Engine.ChildActorComponent|GetChildActor _actorcomponent
                (:then
                  (if (Variables|Private|GetMoveUp?)
                    (if (>= (Variables|Private|GetuseLength) (Spline|GetSplineLength (Variables|Default|GetSpline)))
                      (if (Variables|Param/Move|GetActorWhenMoveIsReverse?)
                        (Variables|Private|SetMoveUp? false)
                        (Utilities|MMoveSetRotation)
                        (else
                          (Actor|DestroyActor (Variables|/Script/Engine.ChildActorComponent|GetChildActor (Variables|Default|GetActorComponent)))))
                      (else
                        (if (and (> (Variables|Param/Move|GetDelayBeforeMoveFrontEndPoint) 0.0) (<= (Variables|Private|GetuseLength) 0.0))
                          (Utilities|FlowControl|Delay (Variables|Param/Move|GetDelayBeforeMoveFrontEndPoint)))
                        (Variables|Private|SetuseLength (+ (Variables|Private|GetuseLength) (Variables|Private|GetDelta)))
                        (Transformation|SetRelativeLocation (Variables|Default|GetActorComponent) (Spline|GetLocationatDistanceAlongSpline (Variables|Default|GetSpline) (Variables|Private|GetuseLength) "Local") false false :!label _label)
                        (Transformation|SetWorldLocation (Variables|Default|GetActorComponent) (Spline|FindLocationClosesttoWorldLocation (Variables|Default|GetSpline) (Transformation|GetWorldLocation (Variables|Default|GetActorComponent)) "World") false false)))
                    (elif (Variables|Param/Move|GetActorWhenMoveIsReverse?)
                      (if (<= (Variables|Private|GetuseLength) 0.0)
                        (Variables|Private|SetMoveUp? true)
                        (Utilities|MMoveSetRotation)
                        (else
                          (Variables|Private|SetuseLength (- (Variables|Private|GetuseLength) (Variables|Private|GetDelta)))
                          (goto _label))))))
                (:else
                  (if (Variables|Param/Move|GetSpawnActorWhenDestroy?)
                    (Utilities|FlowControl|Delay (Variables|Param/Move|GetDelayForSpawnNewActor))
                    (bind _returnvalue (AddComponent|AddChildActorComponent false (Math|Transform|MakeTransform (Transformation|GetWorldLocation (Variables|Default|GetSpline)) "0, 0, 0" (Variables|Param/Move|GetWorldScale))))
                    (bind _output_get (Variables|Default|SetActorComponent _returnvalue))
                    (ChildActorComponent|SetChildActorClass _output_get (Variables|Param/Move|GetActorForMove))
                    (Variables|Private|SetuseLength 0.0)
                    (goto _label)))))
            (:else)))
        (:else)))))

(event Custom|Ev_Active
  (params (Active? :type Boolean))
  (bind _actorcomponent (Variables|Default|GetActorComponent))
  (bind _audio (Variables|Default|GetAudio))
  (Variables|Param|SetActive? Active?)
  (if (Variables|Param|GetActive?)
    (Utilities|FlowControl|Sequence
      (:then_0
        (bind _particlesystem (Variables|Default|GetParticleSystem)
          (:then
            (Effects|Components|ParticleSystem|SetTemplate _particlesystem (Variables|Param|GetParticaleSystem)))
          (:else)))
      (:then_2
        (bind _sound (Variables|Param/Audio|GetSound)
          (:then
            (Audio|Components|Audio|SetSound _audio _sound)
            (Components|Activation|SetAutoActivate _audio (Variables|Param/Audio|GetSoundAutoActivate?))
            (Variables|/Script/Engine.AudioComponent|SetAttenuationSettings (Variables|Default|GetAudio) (Variables|Param/Audio|GetSound_AttentionSettings)))
          (:else)))
      (:then_3
        (bind _sprite (Variables|Param|GetSprite)
          (:then
            (Rendering|Components|Sprite|SetSprite (Variables|Default|GetPaperSprite) _sprite))
          (:else)))
      (:then_4
        (bind _actorformove (Variables|Param/Move|GetActorForMove)
          (:then
            (ChildActorComponent|SetChildActorClass _actorcomponent _actorformove)
            (Variables|/Script/Engine.ChildActorComponent|GetChildActor _actorcomponent
              (:then
                (Transformation|SetWorldScale3D _actorcomponent (Variables|Param/Move|GetWorldScale)))
              (:else)))
          (:else))))))

(event EventBeginPlay
  (CallFunction|FConstruction))