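; BP_MoveBox is a box actor that shifts when the player touches its trigger components.
; Begin-overlap events on Box1 and BC_2 ask the other actor through an interface whether it is the player.
; If so, PSBox takes a small, fixed, unswept step along local X; otherwise the overlapping actor or component name is printed.
; Its GetActorID and OpenDoor interface functions only return constants.
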(event OnComponentBeginOverlap(BC_2)
  (params (OverlappedComponent :type Primitive%20Component%20Object%20Reference) (OtherActor :type Actor%20Object%20Reference) (OtherComp :type Primitive%20Component%20Object%20Reference) (OtherBodyIndex :type Integer) (bFromSweep :type Boolean) (SweepResult :type Hit%20Result%20Structure%20%28by%20ref%29))
  (bind _isplayer_ (Class|BPIPlayer|BPIIsPlayer?(Message) OtherActor))
  (if _isplayer_
    (Transformation|AddLocalOffset (Variables|Default|GetPS_Box) "5.000000,0.000000,0.000000" false false)
    (else
      (Development|PrintString (Utilities|GetDisplayName OtherComp)))))

(event OnComponentBeginOverlap(Box1)
  (params (OverlappedComponent :type Primitive%20Component%20Object%20Reference) (OtherActor :type Actor%20Object%20Reference) (OtherComp :type Primitive%20Component%20Object%20Reference) (OtherBodyIndex :type Integer) (bFromSweep :type Boolean) (SweepResult :type Hit%20Result%20Structure%20%28by%20ref%29))
  (bind _isplayer_ (Class|BPIPlayer|BPIIsPlayer?(Message) OtherActor))
  (if _isplayer_
    (Transformation|AddLocalOffset (Variables|Default|GetPS_Box) "5.000000,0.000000,0.000000" false false)
    (else
      (Development|PrintString (Utilities|GetDisplayName OtherActor)))))

(event EventBeginPlay)

(event Collision|EventActorBeginOverlap
  (params (OtherActor :type Actor%20Object%20Reference)))

(event EventTick
  (params (DeltaSeconds :type Float%20%28single-precision%29)))

(fn ConstructionScript)

(fn BPIGetActorID
  (return 0))

(fn BPIOpenDoor
  (return true))