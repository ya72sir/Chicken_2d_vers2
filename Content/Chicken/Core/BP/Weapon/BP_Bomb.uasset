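; BP_Bomb is a bomb weapon actor that damages the player or the cockroach boss on contact, then explodes.
; Tick spins the bomb particle, and its audio cue replays itself until stopped.
; Sphere overlap identifies the player by interface message or the boss by cast, ignoring anything else, and applies point damage.
; Both hits share Ev_BombExplosion's sequence: activate explosion particles, hide the bomb, disable collision, silence audio, destroy after a short delay.
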(event OnComponentBeginOverlap(SphColl_DamagePlayer)
  (params (OverlappedComponent :type Primitive%20Component%20Object%20Reference) (OtherActor :type Actor%20Object%20Reference) (OtherComp :type Primitive%20Component%20Object%20Reference) (OtherBodyIndex :type Integer) (bFromSweep :type Boolean) (SweepResult :type Hit%20Result%20Structure%20%28by%20ref%29))
  (bind _damage (Variables|Default|GetDamage))
  (bind (_isplayer_ _player) (Class|BPIPlayer|BPIIsPlayer?(Message) OtherActor))
  (if _isplayer_
    (Game|Damage|ApplyPointDamage _player _damage (Math|Vector|MakeVector 3.0 3.0 3.0) (Collision|MakeHitResult false false 0.0 0.0 "0, 0, 0" "0, 0, 0" "0,0,1" "0,0,1" 0 0))
    (else
      (bind _ascockroach_boss (Utilities|Casting|CastToCockroach_Boss OtherActor))
      (Game|Damage|ApplyPointDamage _ascockroach_boss _damage (Math|Vector|MakeVector 3.0 3.0 3.0) (Collision|MakeHitResult false false 0.0 0.0 "0, 0, 0" "0, 0, 0" "0,0,1" "0,0,1" 0 0))))
  (Components|Activation|SetActive (Variables|Default|GetPS_BombExplosion) true false)
  (Rendering|SetVisibility (Variables|Default|GetPSComp_Bomb) false false)
  (Collision|SetActorEnableCollision false)
  (Audio|Components|Audio|Stop (Variables|Default|GetFlowStar_Cue))
  (Variables|Default|SetStopSound true)
  (Utilities|FlowControl|Delay 1.0)
  (Actor|DestroyActor))

(event OnAudioFinished(FlowStar_Cue)
  (if (not (Variables|Default|GetStopSound))
    (Audio|Components|Audio|Play (Variables|Default|GetFlowStar_Cue) 0.0)))

(event Custom|Ev_BombExplosion
  (Components|Activation|SetActive (Variables|Default|GetPS_BombExplosion) true false)
  (Rendering|SetVisibility (Variables|Default|GetPSComp_Bomb) false false)
  (Collision|SetActorEnableCollision false)
  (Audio|Components|Audio|Stop (Variables|Default|GetFlowStar_Cue))
  (Variables|Default|SetStopSound true)
  (Utilities|FlowControl|Delay 1.0)
  (Actor|DestroyActor))

(event EventTick
  (params (DeltaSeconds :type Float%20%28single-precision%29))
  (Transformation|AddLocalRotation (Variables|Default|GetPSComp_Bomb) (Math|Vector|RotatorfromAxisandAngle "0.000000,1.000000,0.000000" (* DeltaSeconds 5e+02)) false false))

(fn ConstructionScript)