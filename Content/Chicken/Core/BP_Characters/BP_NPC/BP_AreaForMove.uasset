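; BP_AreaForMove is an area actor that moves an NPC back and forth along a spline, spawning a Cockroach_Mini if none is set.
; Tick advances distance along the spline at Speed, flipping direction and rotation at each end.
; With ActiveIsBoxTrigger on, a player entering the box starts movement while the enemy passes death-state checks.
; Once the player leaves, movement finishes the current leg; with the trigger off, it runs continuously.
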(event OnComponentBeginOverlap(Box)
  (params (OverlappedComponent :type Primitive%20Component%20Object%20Reference) (OtherActor :type Actor%20Object%20Reference) (OtherComp :type Primitive%20Component%20Object%20Reference) (OtherBodyIndex :type Integer) (bFromSweep :type Boolean) (SweepResult :type Hit%20Result%20Structure%20%28by%20ref%29))
  (bind (_activeenemyfordead_ _enemydead_) (Class|BPINPC|BPINPCIsDead?(Message) (Variables|Default|GetEnemys)))
  (if _activeenemyfordead_
    (if (not _enemydead_)
      (if (Variables|Default|GetActiveIsBoxTrigger?)
        (bind (_isplayer_ _player) (Class|BPIPlayer|BPIIsPlayer?(Message) OtherActor))
        (if _isplayer_
          (Variables|Default|SetBP_Player _player)
          (Variables|Default|SetMove? true))))))

(event OnComponentEndOverlap(Box)
  (params (OverlappedComponent :type Primitive%20Component%20Object%20Reference) (OtherActor :type Actor%20Object%20Reference) (OtherComp :type Primitive%20Component%20Object%20Reference) (OtherBodyIndex :type Integer))
  (bind _isplayer_ (Class|BPIPlayer|BPIIsPlayer?(Message) OtherActor))
  (if _isplayer_
    (Variables|Default|SetBP_Player 0)))

(event EventBeginPlay
  (Variables|Default|GetEnemys
    (:then)
    (:else
      (bind _returnvalue (Game|SpawnActorfromClass "/Game/Chicken/Core/BP_Characters/BP_NPC/Enemys/Cockroach_Mini.Cockroach_Mini_C" (Math|Transform|MakeTransform "0, 0, 0") "AlwaysSpawn" 0 0))
      (Variables|Default|SetEnemys _returnvalue))))

(event EventTick
  (params (DeltaSeconds :type Float%20%28single-precision%29))
  (Variables|Default|GetEnemys
    (:then
      (Variables|Default|GetBP_Player
        (:then
          (CallFunction|FMove DeltaSeconds :!label _label))
        (:else
          (if (Variables|Default|GetActiveIsBoxTrigger?)
            (if (Variables|Default|GetMove?)
              (goto _label))
            (else
              (goto _label))))))
    (:else)))

(fn ConstructionScript)

(fn FMove
  (params (Tick :type Float%20%28single-precision%29))
  (LocalVariables|SetLSpeed (* Tick (Variables|Default|Getspeed)))
  (if (Variables|Default|GetDirectionMoveUp?)
    (if (>= (Variables|Default|GetuseLength) (Spline|GetSplineLength (Variables|Default|GetSpline)))
      (Variables|Default|SetDirectionMoveUp? false)
      (Transformation|SetActorRotation (Variables|Default|GetEnemys) (select (Variables|Default|GetDirectionMoveUp?) "0, 0, 0" "0,-180.000000, 0") :!label _label)
      (Variables|Default|SetMove? false)
      (else
        (Variables|Default|SetuseLength (+ (Variables|Default|GetuseLength) (LocalVariables|GetLSpeed)))
        (Transformation|SetActorLocation (Variables|Default|GetEnemys) (Spline|GetLocationatDistanceAlongSpline (Variables|Default|GetSpline) (Variables|Default|GetuseLength) "World") false false :!label _label_2)))
    (elif (<= (Variables|Default|GetuseLength) 0.0)
      (Variables|Default|SetDirectionMoveUp? true)
      (goto _label)
      (else
        (Variables|Default|SetuseLength (- (Variables|Default|GetuseLength) (LocalVariables|GetLSpeed)))
        (goto _label_2)))))