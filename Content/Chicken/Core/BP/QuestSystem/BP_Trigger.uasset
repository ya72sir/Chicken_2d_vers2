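; Quest trigger volume that signals quest disabling when the player enters its box.
; An NPC interface event assigns its quest ID, which the disable-quest function returns.
; On player overlap, checked through an interface, it calls that function to start self-destruction after a short delay, then notifies the game mode.
; The actor ID, NPC death and door interface functions return only default values.
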(event OnComponentBeginOverlap(Box)
  (params (OverlappedComponent :type Primitive%20Component%20Object%20Reference) (OtherActor :type Actor%20Object%20Reference) (OtherComp :type Primitive%20Component%20Object%20Reference) (OtherBodyIndex :type Integer) (bFromSweep :type Boolean) (SweepResult :type Hit%20Result%20Structure%20%28by%20ref%29))
  (bind _isplayer_ (Class|BPIPlayer|BPIIsPlayer?(Message) OtherActor))
  (if _isplayer_
    (CallFunction|BPINPCDisableQuest)
    (Default|EvDisableQuest (CallFunction|BFLGetGameModeBP))))

(event Custom|Ev_DestoryActor
  (Utilities|FlowControl|Delay 0.2)
  (Actor|DestroyActor))

(event EventBPINPCSetIdDialogandSetIdQuest
  (params (ID%20For%20Dialog%20System :type Integer) (ID%20For%20Quest%20System :type Integer))
  (Variables|Default|SetIdQuestSys ID%20For%20Quest%20System))

(fn ConstructionScript)

(fn BPIGetActorID
  (return 0))

(fn BPINPCDisableQuest
  (CallFunction|EvDestoryActor)
  (return (Variables|Default|GetIdQuestSys)))

(fn BPINPCIsDead?
  (return false false))

(fn BPIOpenDoor
  (return false))