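; BP_DoorKeys is a Paper2D locked door that opens when a player carrying its matching key enters the trigger.
; Construction looks up the key type in DT_Keys to set the lock sprites and key data.
; On overlap, it queries the player through interface calls, then drops blocking collision, plays an opening flipbook and shows a replacement door sprite.
; Without the key, it shows the player a key name and icon message.
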(event OnComponentBeginOverlap(BC_OpenDoorForKey)
  (params (OverlappedComponent :type Primitive%20Component%20Object%20Reference) (OtherActor :type Actor%20Object%20Reference) (OtherComp :type Primitive%20Component%20Object%20Reference) (OtherBodyIndex :type Integer) (bFromSweep :type Boolean) (SweepResult :type Hit%20Result%20Structure%20%28by%20ref%29))
  (bind (_isplayer_ _player) (Class|BPIPlayer|BPIIsPlayer?(Message) OtherActor))
  (if _isplayer_
    (Variables|Default|SetBP_Player _player)
    (CallFunction|EvOpenDoor)))

(event OnComponentEndOverlap(BC_OpenDoorForKey)
  (params (OverlappedComponent :type Primitive%20Component%20Object%20Reference) (OtherActor :type Actor%20Object%20Reference) (OtherComp :type Primitive%20Component%20Object%20Reference) (OtherBodyIndex :type Integer))
  (bind _isplayer_ (Class|BPIPlayer|BPIIsPlayer?(Message) OtherActor))
  (if _isplayer_
    (Variables|Default|SetBP_Player 0)))

(event Custom|Ev_OpenDoor
  (bind _paramkey (Variables|Private_ParamKey|GetparamKey))
  (bind _bc_blockdoor (Variables|Default|GetBC_BlockDoor))
  (bind _pf_opendoor (Variables|Default|GetPF_OpenDoor))
  (bind (_id _name _ps_key) (Utilities|Struct|BreakStr_Key _paramkey))
  (bind _find_ (Default|BPIFindKey (Variables|Default|GetBP_Player) (Variables|Default|GetNameKeyForOpenDoor)))
  (if _find_
    (if (Variables|/Script/Engine.SceneComponent|GetbVisible (Variables|Default|GetCompPS_Door))
      (Rendering|SetVisibility (Variables|Default|GetCompPS_Door) false false)
      (Collision|SetCollisionEnabled _bc_blockdoor "NoCollision")
      (bind _returnvalue (Sprite|SetFlipbook (Variables|Default|GetCompPF_OpenDoor) _pf_opendoor))
      (if _returnvalue
        (Rendering|Components|Sprite|SetSprite (Variables|Default|GetPaperSprite) (Variables|Default|GetPS_CastleOpen))
        (Utilities|FlowControl|Delay (Class|PaperFlipbook|GetTotalDuration _pf_opendoor))
        (Sprite|SetFlipbook (Variables|Default|GetCompPF_OpenDoor))
        (Rendering|SetVisibility (Variables|Default|GetCompPS_DoorCloose) true false)
        (Rendering|SetVisibility (Variables|Default|GetPaperSprite) false false)))
    (else
      (Rendering|SetVisibility _bc_blockdoor true false)
      (Default|BPIShowMessage (Variables|Default|GetBP_Player) (Utilities|Text|FormatText "You found the key - {nameKey}" (Utilities|Text|ToText(String) _name)) _ps_key))))

(fn ConstructionScript
  (Rendering|Components|Sprite|SetSprite (Variables|Default|GetCompPS_Door) (Variables|Default|GetPS_DoorClose))
  (bind _returnvalue (Utilities|GetDataTableRow "/Game/Chicken/Core/DataTable/DT_Keys.DT_Keys" (Utilities|String|StringToName (Utilities|String|EnumtoString (Variables|Default|GetNameKeyForOpenDoor))))
    (:then
      (bind _output_get (Variables|Private_ParamKey|SetparamKey _returnvalue))
      (Rendering|Components|Sprite|SetSprite (Variables|Default|GetPaperSprite) (.PS_CastleClose (Utilities|Struct|BreakStr_Key _output_get)))
      (Variables|Default|SetPS_CastleOpen (.PS_CastleOpen (Utilities|Struct|BreakStr_Key _output_get))))))

(fn BPIGetActorID
  (return 0))

(fn BPIOpenDoor
  (return false))