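; BP_PlayerState tracks the money the player collects on the current level and shows it on the HUD.
; On BeginPlay it registers with the player controller, reads the level's money maximum from DT_DataLevels and restores any stored amount from the game instance.
; An add event increments money by one, then refreshes the HUD money widget, clamping only the displayed value to that maximum.
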(event Custom|Ev_AddMoney
  (Math|Integer|IncrementInt (Variables|Default|GetMoney)
    (:%20%20
      (CallFunction|EvShowMoney))))

(event Custom|Ev_ShowMoney
  (bind _wbp_hud (Variables|/Game/Chicken/Core/BP_Characters/BP_Player/Level/BP_HUD.BP_HUD_C|GetWBP_HUD (CallFunction|BFLGetHUD))
    (:then
      (Default|FShowMoney (Variables|/Game/Chicken/Core/BP_Widgets/HUD/WBP_HUD.WBP_HUD_C|GetWBP_Money _wbp_hud) (Math|Integer|Clamp(Integer) (Variables|Default|GetMoney) 0 (Variables|Default|GetMoney_Max)) (Variables|Default|GetMoney_Max)))
    (:else)))

(event EventBeginPlay
  (bind _asbp_game_instance (CallFunction|BFLGetGameInstanceBP))
  (bind _currentmap (Default|FGetCurrentLevel _asbp_game_instance))
  (bind (_money _returnvalue) (Default|FGetPlayerParamMoneywithLevel _asbp_game_instance _currentmap))
  (Default|EvSetBPPlayerState (CallFunction|BFLGetPlayerControllerBP) self)
  (bind _returnvalue_2 (Utilities|GetDataTableRow "/Game/Chicken/Core/DataTable/DT_DataLevels.DT_DataLevels" (Utilities|String|StringToName (Utilities|String|EnumtoString (Default|FGetCurrentLevel (CallFunction|BFLGetGameInstanceBP)))))
    (:then
      (Variables|Default|SetMoney_Max (.MoneyOnLevel_MaxCound (Utilities|Struct|BreakStrDataLevels _returnvalue_2))))
    (:RowNotFound
      _))
  (if _returnvalue
    (Variables|Default|SetMoney _money)
    (CallFunction|EvShowMoney)))

(fn ConstructionScript)