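; Spline-mover child Blueprint for the cockroach boss encounter, built on the BP_MasterForSpline parent logic.
; A player entering the box starts movement; leaving clears the player and sets direction to MoveUp, and without a player Tick allows movement only in that direction.
; When the child actor reports death, a DoOnce explodes and destroys all ActorsForDamage, then spawns SpawnActorClass with an explosion at a hardcoded location.
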(event OnComponentBeginOverlap(Box)
  (params (OverlappedComponent :type Primitive%20Component%20Object%20Reference) (OtherActor :type Actor%20Object%20Reference) (OtherComp :type Primitive%20Component%20Object%20Reference) (OtherBodyIndex :type Integer) (bFromSweep :type Boolean) (SweepResult :type Hit%20Result%20Structure%20%28by%20ref%29))
  (bind (_isplayer_ _player) (Class|BPIPlayer|BPIIsPlayer?(Message) OtherActor))
  (if _isplayer_
    (Variables|Default|SetBP_Player _player)
    (Variables|Default|SetActorIsMove? true)))

(event OnComponentEndOverlap(Box)
  (params (OverlappedComponent :type Primitive%20Component%20Object%20Reference) (OtherActor :type Actor%20Object%20Reference) (OtherComp :type Primitive%20Component%20Object%20Reference) (OtherBodyIndex :type Integer))
  (bind _isplayer_ (Class|BPIPlayer|BPIIsPlayer?(Message) OtherActor))
  (if _isplayer_
    (Variables|Default|SetBP_Player 0)
    (Variables|Default|SetCurrentDirection (Variables|Default|GetMoveUp?))))

(event EventBeginPlay
  (|CallParentFunction))

(event Collision|EventActorBeginOverlap
  (params (OtherActor :type Actor%20Object%20Reference)))

(event EventTick
  (params (DeltaSeconds :type Float%20%28single-precision%29))
  (bind _returnvalue (Math|Vector|MakeVector -1025.0 5.0 -7.3e+02))
  (bind _actorsfordamage (Variables|Default|GetActorsForDamage))
  (|CallParentFunction DeltaSeconds)
  (Utilities|FlowControl|Sequence
    (:then_0
      (Variables|Default|GetBP_Player
        (:then)
        (:else
          (if (Math|Boolean|Equal(Boolean) (Variables|Default|GetCurrentDirection) (Variables|Default|GetMoveUp?))
            (Variables|Default|SetActorIsMove? true)
            (else
              (Variables|Default|SetActorIsMove? false))))))
    (:then_1
      (bind _childactor (Variables|/Script/Engine.ChildActorComponent|GetChildActor (Variables|Default|GetActorComponent))
        (:then
          (bind _enemydead_ (Class|BPINPC|BPINPCIsDead?(Message) _childactor))
          (if _enemydead_
            (Utilities|FlowControl|DoOnce false
              (:Completed
                (for _array_element _actorsfordamage
                  (Effects|SpawnEmitteratLocation "/Game/Chicken/MaterialLibrary/Particles/PS_BombExplosion.PS_BombExplosion" (Transformation|GetActorLocation _array_element) "0, 0,90.000000")
                  (Actor|DestroyActor _array_element))
                (Utilities|Array|Clear _actorsfordamage)
                (Game|SpawnActorfromClass (Variables|Default|GetSpawnActorClass) (Math|Transform|MakeTransform _returnvalue) "AlwaysSpawn" 0 "NewEnumerator3" 0)
                (Effects|SpawnEmitteratLocation "/Game/Chicken/MaterialLibrary/Particles/PS_BombExplosion.PS_BombExplosion" _returnvalue "0, 0,90.000000")))))
        (:else)))))

(fn ConstructionScript
  (|CallParentFunction))