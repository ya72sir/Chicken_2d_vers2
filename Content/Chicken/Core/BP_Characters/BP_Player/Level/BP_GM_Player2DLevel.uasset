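; Game mode for 2D levels, handling intro cutscene, start, game over, restart, completion and removal of Bitcoin pickups from saved counts.
; It runs a linear quest chain from per-level DataTables, where Dialog, Attack and Trigger quests advance an ID until Level Completed.
; Activation spawns quest actors and updates the HUD.
; Finished dialogs can unlock double jump, activate actors and tour camera points before loading the next quest.
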(event Custom|Ev_GameOver
  (bind _asbp_player_controller (CallFunction|BFLGetPlayerControllerBP))
  (Utilities|Time|SetGlobalTimeDilation 0.15)
  (Utilities|FlowControl|Delay 0.5)
  (Utilities|Time|SetGlobalTimeDilation 1.0)
  (Game|SetGamePaused true)
  (Default|EvWBPFinishGame _asbp_player_controller)
  (Default|EvShowCurrentWBP _asbp_player_controller))

(event Custom|Ev_Restart
  (Default|EvRestartGameLevel (CallFunction|BFLGetGameInstanceBP)))

(event Custom|Ev_StartGame
  (if (Utilities|Enum|NotEqual(Enum) (Default|FGetCurrentLevel (CallFunction|BFLGetGameInstanceBP)) "NewEnumerator0")
    (Class|GameModeBase|RestartPlayer (CallFunction|BFLGetPlayerControllerBP))
    (Default|EvStartPlayTimer (CallFunction|BFLGetGameState))
    (CallFunction|EvLoadDTforQuestSystem)))

(event Custom|Ev_LevelComplited
  (Default|EvLevelComplited (CallFunction|BFLGetHUD))
  (Default|EvLevelComplited (CallFunction|BFLGetGameInstanceBP)))

(event Custom|Ev_PlayDefaultIntroCutscene
  (bind _outactors (Actor|GetAllActorsOfClass "/Script/LevelSequence.LevelSequenceActor"))
  (if (Utilities|Array|IsValidIndex _outactors)
    (Default|EvPlaySkippableCutscene (CallFunction|BFLGetPlayerControllerBP) (Variables|/Script/LevelSequence.LevelSequenceActor|GetSequencePlayer (Utilities|Array|Get(acopy) _outactors)))
    (else
      (CallFunction|EvStartGame))))

(event EventBeginPlay
  (Utilities|IsValid (CallFunction|BFLGetGameInstanceBP)
    (:Is%20Valid
      (CallFunction|FInitialize)
      (CallFunction|EvPlayDefaultIntroCutscene))
    (:Is%20Not%20Valid
      (Development|PrintString "InstanceNotValid" true true "(R=1.000000,G=0.000000,B=0.032916,A=1.000000)"))))

(event Custom|Ev_ActivateQuest
  (if (Utilities|Enum|NotEqual(Enum) (Default|FGetCurrentLevel (CallFunction|BFLGetGameInstanceBP)) "NewEnumerator0")
    (|ActivateQuest)))

(event Custom|Ev_GetDataTableForCurrentQuests
  (bind _asbp_game_instance (CallFunction|BFLGetGameInstanceBP))
  (bind _currentmap (Default|FGetCurrentLevel _asbp_game_instance))
  (Utilities|IsValid _asbp_game_instance
    (:Is%20Valid
      (if (Utilities|Enum|NotEqual(Enum) _currentmap "NewEnumerator0")
        (bind _returnvalue (Utilities|GetDataTableRow "/Game/Chicken/Core/DataTable/Quests/DT_LevelForDataTable.DT_LevelForDataTable" (Utilities|String|StringToName (Utilities|String|EnumtoString _currentmap)))
          (:then
            (Variables|Default|SetDataTable_CurrentQuest (.DataTableQuestName (Utilities|Struct|BreakStrLevelForDataTable _returnvalue)))
            (Variables|Default|SetDataTable_CurrentDialogSys (.DataTableDialogName (Utilities|Struct|BreakStrLevelForDataTable _returnvalue)))))))))

(event Custom|Ev_LoadDTForQuestSystem
  (if (!= (Variables|QuestSystem|GetQuest_CompletedID) (Variables|QuestSystem|GetQuest_CurrentID))
    (Variables|QuestSystem|SetQuest_CurrentID (Variables|QuestSystem|GetQuest_CompletedID))
    (bind _datatable_currentquest (Variables|Default|GetDataTable_CurrentQuest)
      (:then
        (bind _returnvalue (Utilities|GetDataTableRow _datatable_currentquest (Utilities|String|StringToName (Utilities|String|ToString(Integer) (Variables|QuestSystem|GetQuest_CompletedID))))
          (:then
            (bind _output_get (Variables|QuestSystem|SetQuest_Data _returnvalue))
            (CallFunction|EvActivateQuest)
            (switch Utilities|FlowControl|Switch|SwitchonEQuestInform (.TypeQuest (Utilities|Struct|BreakStrQuestSys _output_get))
              (:NewEnumerator3
                (Default|EvLevelComplited (CallFunction|BFLGetPlayerControllerBP)))))))
      (:else))))

(event Custom|Ev_DisableQuest
  (switch Utilities|FlowControl|Switch|SwitchonEQuestInform (.TypeQuest (Utilities|Struct|BreakStrQuestSys (Variables|QuestSystem|GetQuest_Data)))
    (:NewEnumerator0
      (|Dialog))
    (:NewEnumerator1
      (Math|Integer|IncrementInt (Variables|QuestSystem|GetQuest_CompletedID) :!label _label
        (:%20%20
          (CallFunction|EvLoadDTforQuestSystem))))
    (:NewEnumerator2
      (goto _label))))

(event Custom|Ev_ShowDialog_QuestAttack
  (params (OwnerDialogSys :type Actor%20Object%20Reference))
  (Default|EvWBPDialog (CallFunction|BFLGetPlayerControllerBP) OwnerDialogSys))

(event Custom|Ev_LoadMoney
  (bind _asbp_game_instance (CallFunction|BFLGetGameInstanceBP))
  (bind _currentmap (Default|FGetCurrentLevel _asbp_game_instance))
  (bind (_money _returnvalue) (Default|FGetPlayerParamMoneywithLevel _asbp_game_instance _currentmap))
  (if _returnvalue
    (for _index (range 1 _money)
      (bind _outactors (Actor|GetAllActorsOfClass "/Game/Chicken/Core/BP/BP_MasterForSpline/ActorsForSpline/BP_MoneyBitcoin.BP_MoneyBitcoin_C"))
      (Default|EvDestroyMoney (Utilities|Array|Get(acopy) _outactors (Math|Random|RandomInteger (- (Utilities|Array|Length _outactors) 1)))))))

(fn ConstructionScript)

(fn FInitialize
  (Variables|AIForPlayer|SetBP_PlayerController (CallFunction|BFLGetPlayerControllerBP))
  (Variables|AIforPlayer|SetBP_Player2D (CallFunction|BFLGetPlayerCharacterBP))
  (Default|EvCreateHUD (CallFunction|BFLGetHUD))
  (CallFunction|EvGetDataTableforCurrentQuests)
  (CallFunction|EvLoadMoney))

(event Custom|Ev_GoToCamera
  (bind _bp_player2d (CallFunction|BFLGetPlayerCharacterBP))
  (bind _pointsforvector (Variables|Default|GetPointsForVector))
  (bind _returnvalue (Utilities|Array|Length _pointsforvector))
  (Default|EvDisableMoveCharacter (CallFunction|BFLGetPlayerControllerBP) true)
  (if (!= _returnvalue -1)
    (if (< (Variables|Default|GetId_VectorPoint) _returnvalue)
      (Default|EvCameraGo _bp_player2d (Utilities|Array|Get(acopy) _pointsforvector (Variables|Default|GetId_VectorPoint)))
      (Math|Integer|IncrementInt (Variables|Default|GetId_VectorPoint)
        (:%20%20
          (goto _label Reset)))
      (else
        (Variables|Default|SetTimerMessage 2.0)
        (Utilities|FlowControl|RetriggerableDelay (Variables|Default|GetTimerMessage))
        (Default|EvCameraMoveExit _bp_player2d)
        (Utilities|FlowControl|DoOnce false :!label _label
          (:Completed
            (Math|Integer|IncrementInt (Variables|QuestSystem|GetQuest_CompletedID)
              (:%20%20
                (CallFunction|EvLoadDTforQuestSystem)
                (Variables|Default|SetId_VectorPoint 0)
                (Default|EvDisableMoveCharacter (CallFunction|BFLGetPlayerControllerBP) false)
                (CallFunction|EvResetDoOnce)))))))))

(event Custom|Ev_ExitCameraGoToPoints
  (Variables|Default|SetTimerMessage 0.0)
  (Utilities|FlowControl|RetriggerableDelay (Variables|Default|GetTimerMessage))
  (Default|EvCameraMoveExit (CallFunction|BFLGetPlayerCharacterBP))
  (Utilities|FlowControl|DoOnce false
    (:Completed
      (Math|Integer|IncrementInt (Variables|QuestSystem|GetQuest_CompletedID)
        (:%20%20
          (CallFunction|EvLoadDTforQuestSystem)
          (Variables|Default|SetId_VectorPoint 0)
          (Default|EvDisableMoveCharacter (CallFunction|BFLGetPlayerControllerBP) false)
          (CallFunction|EvResetDoOnce))))))

(event Custom|Ev_ResetDoOnce
  (Utilities|FlowControl|DoOnce false) ; enters at Reset
)