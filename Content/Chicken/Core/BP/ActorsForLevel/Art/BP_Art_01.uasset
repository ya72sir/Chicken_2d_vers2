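; BP_Art_01 is a level art actor that reacts with sound, particles and a scale animation when the player overlaps its capsule.
; A player check through BPIIsPlayerMessage starts the sound cue, particle system and a timeline that drives the actor's X and Y scale, keeping Z at 1.
; An Active flag blocks retriggering until the timeline finishes, which also switches the particles off.
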(event OnComponentBeginOverlap(Capsule)
  (params (OverlappedComponent :type Primitive%20Component%20Object%20Reference) (OtherActor :type Actor%20Object%20Reference) (OtherComp :type Primitive%20Component%20Object%20Reference) (OtherBodyIndex :type Integer) (bFromSweep :type Boolean) (SweepResult :type Hit%20Result%20Structure%20%28by%20ref%29))
  (if (not (Variables|Default|GetbActive?))
    (bind (_isplayer_ _player) (Class|BPIPlayer|BPIIsPlayer?(Message) OtherActor))
    (if _isplayer_
      (Variables|Default|SetBP_Player _player)
      (Variables|Default|SetbActive? true)
      (Audio|Components|Audio|Play (Variables|Default|Getdzzz_Cue) 0.0)
      (Components|Activation|SetActive (Variables|Default|GetParticleSystem) true false)
      (bind _newtrack_0 (Timeline|Timeline_0 PlayFromStart)
        (:Update
          (Transformation|SetActorScale3D (Math|Vector|MakeVector _newtrack_0 _newtrack_0 1.0)))
        (:Finished
          (Variables|Default|SetbActive? false)
          (Components|Activation|SetActive (Variables|Default|GetParticleSystem) false false))))))

(fn ConstructionScript)