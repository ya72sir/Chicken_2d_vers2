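; Button-operated door that opens when the player, or an actor answering the open-door interface message, overlaps its trigger box.
; It responds only while active, a state switched on through the activate-actor interface event.
; Pressing swaps the switch sprite, plays audio and runs a timeline that lowers the door component.
; With Revers set, delays precede restoring the sprite and reversing the timeline, re-arming the button.
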(event OnComponentBeginOverlap(Box)
  (params (OverlappedComponent :type Primitive%20Component%20Object%20Reference) (OtherActor :type Actor%20Object%20Reference) (OtherComp :type Primitive%20Component%20Object%20Reference) (OtherBodyIndex :type Integer) (bFromSweep :type Boolean) (SweepResult :type Hit%20Result%20Structure%20%28by%20ref%29))
  (if (Variables|Default|GetbActorIsActive?)
    (bind _isplayer_ (Class|BPIPlayer|BPIIsPlayer?(Message) OtherActor))
    (if _isplayer_
      (if (not (Variables|Default|GetbActive?)) :!label _label
        (Variables|Default|SetbActive? true)
        (Rendering|Components|Sprite|SetSprite (Variables|Default|GetPaperSprite_Switch) (Variables|Default|GetFinishButton))
        (Audio|Components|Audio|Play (Variables|Default|GetAudio) 0.0)
        (bind _newtrack_0 (Timeline|Timeline_Door Play)
          (:Update
            (Transformation|SetRelativeLocation (Variables|Default|GetScene1) (Math|Vector|Lerp(Vector) "0, 0, 0" "0, 0,-75.000000" _newtrack_0) false false))
          (:Finished
            (Audio|Components|Audio|Stop (Variables|Default|GetAudio))
            (if (Variables|Default|GetbRevers?)
              (Utilities|FlowControl|Delay 2.0)
              (if (Variables|Default|GetbActive?)
                (Variables|Default|SetbActive? false)
                (Utilities|FlowControl|Delay (Variables|Default|GetFDelay%20before%20closing%20the%20door))
                (Rendering|Components|Sprite|SetSprite (Variables|Default|GetPaperSprite_Switch) (Variables|Default|GetStartButton))
                (Timeline|Timeline_Door Reverse))))))
      (else
        (bind _opendoor_ (Class|BPIItemWorld|BPIOpenDoor(Message) OtherActor))
        (if _opendoor_
          (goto _label))))))

(event EventBPIActivateActor
  (params (ID :type Integer))
  (if (== ID (Variables|Default|GetID))
    (Variables|Default|SetbActorIsActive? true)))

(fn ConstructionScript
  (bind _switchlocation (Variables|Default|GetswitchLocation))
  (Transformation|SetRelativeLocation (Variables|Default|GetPaperSprite_Switch) (Math|Vector|MakeVector (.x _switchlocation) (.y _switchlocation) (.z _switchlocation)) false false)
  (Rendering|Components|Sprite|SetSprite (Variables|Default|GetPaperSprite_Switch) (Variables|Default|GetStartButton))
  (Variables|Default|SetCustomTimeDilation (Variables|Default|GetFCustomTimeDilation)))

(fn BPIGetActorID
  (return 0))

(fn BPIOpenDoor
  (return false))