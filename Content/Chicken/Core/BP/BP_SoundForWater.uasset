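; BP_SoundForWater is a placeable water-sound zone that plays a flowing water cue while the player overlaps its spline mesh.
; The construction script stretches the spline mesh along a two-point spline between Start and Finish and aims an arrow along that direction.
; Overlaps identify the player through an interface call, and the cue replays on finishing until exit clears the player reference and stops it.
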(event OnComponentBeginOverlap(SplineMesh)
  (params (OverlappedComponent :type Primitive%20Component%20Object%20Reference) (OtherActor :type Actor%20Object%20Reference) (OtherComp :type Primitive%20Component%20Object%20Reference) (OtherBodyIndex :type Integer) (bFromSweep :type Boolean) (SweepResult :type Hit%20Result%20Structure%20%28by%20ref%29))
  (bind (_isplayer_ _player) (Class|BPIPlayer|BPIIsPlayer?(Message) OtherActor))
  (if _isplayer_
    (Variables|Default|Setplayer _player)
    (Audio|Components|Audio|Play (Variables|Default|GetFlowWater_Cue) 0.0)))

(event OnComponentEndOverlap(SplineMesh)
  (params (OverlappedComponent :type Primitive%20Component%20Object%20Reference) (OtherActor :type Actor%20Object%20Reference) (OtherComp :type Primitive%20Component%20Object%20Reference) (OtherBodyIndex :type Integer))
  (bind _isplayer_ (Class|BPIPlayer|BPIIsPlayer?(Message) OtherActor))
  (if _isplayer_
    (Variables|Default|Setplayer 0)
    (Audio|Components|Audio|Stop (Variables|Default|GetFlowWater_Cue))))

(event OnAudioFinished(FlowWater_Cue)
  (Variables|Default|Getplayer
    (:then
      (Audio|Components|Audio|Play (Variables|Default|GetFlowWater_Cue) 0.0))
    (:else)))

(fn ConstructionScript
  (bind _spline (Variables|Default|GetSpline))
  (Spline|SetLocationatSplinePoint _spline 0 (Variables|Default|GetStart) "Local" true)
  (Spline|SetLocationatSplinePoint _spline 1 (Variables|Default|GetFinish) "Local" true)
  (SplineMesh|SetStartandEnd (Variables|Default|GetSplineMesh) (Variables|Default|GetStart) (Spline|GetTangentatSplinePoint _spline 0 "Local") (Variables|Default|GetFinish) (Spline|GetTangentatSplinePoint _spline 1 "Local") true :!class /Script/Engine.SplineMeshComponent)
  (Transformation|SetRelativeRotation (Variables|Default|GetArrow) (Math|Rotator|FindLookatRotation (Variables|Default|GetStart) (Variables|Default|GetFinish)) false false))