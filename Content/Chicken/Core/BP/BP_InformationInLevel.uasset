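; In-level information Blueprint that displays a hint text suited to the active input device, gamepad or keyboard.
; On BeginPlay it caches the WBP_InformationInLevel from its widget component and sets either the gamepad or keys text, based on the HUD's GamepadIsActive flag.
; Tick compares that flag to the stored value, but both branches rejoin the update, so the text is set again every frame.
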(event EventTick
  (params (DeltaSeconds :type Float%20%28single-precision%29))
  (bind _asbp_hud (CallFunction|BFLGetHUD))
  (bind _gamepadisactive_ (Variables|/Game/Chicken/Core/BP_Characters/BP_Player/Level/BP_HUD.BP_HUD_C|GetGamepadIsActive? _asbp_hud))
  (if (Math|Boolean|NotEqual(Boolean) (Variables|/Game/Chicken/Core/BP_Characters/BP_Player/Level/BP_HUD.BP_HUD_C|GetGamepadIsActive? (CallFunction|BFLGetHUD)) (Variables|Default|GetGamepadIsAcitve?))
    _
    (else
      _))
  (Variables|Default|SetGamepadIsAcitve? _gamepadisactive_)
  (Default|EvSetText (Variables|Default|GetWBP_InformationLevel) (select _gamepadisactive_ (Variables|Default|GetText_GamepadIsActive) (Variables|Default|GetText_KeysIsActive))))

(event EventBeginPlay
  (bind _asbp_hud (CallFunction|BFLGetHUD))
  (bind _gamepadisactive_ (Variables|/Game/Chicken/Core/BP_Characters/BP_Player/Level/BP_HUD.BP_HUD_C|GetGamepadIsActive? _asbp_hud))
  (bind _aswbp_information_in_level (Utilities|Casting|CastToWBP_InformationInLevel (UserInterface|GetUserWidgetObject (Variables|Default|GetWidget))))
  (Variables|Default|SetWBP_InformationLevel _aswbp_information_in_level)
  (Variables|Default|SetGamepadIsAcitve? _gamepadisactive_)
  (Default|EvSetText (Variables|Default|GetWBP_InformationLevel) (select _gamepadisactive_ (Variables|Default|GetText_GamepadIsActive) (Variables|Default|GetText_KeysIsActive))))

(fn ConstructionScript)