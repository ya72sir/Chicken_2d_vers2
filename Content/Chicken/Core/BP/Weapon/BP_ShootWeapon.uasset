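; BP_ShootWeapon is a weapon actor that fires repeatedly while a player is inside its trigger area.
; Overlapping BC_ArreaForShoot checks for a player via an interface message, stores the reference, fires immediately and starts a looping timer, cleared when the player leaves.
; FShoot spawns a BP_Shoot at the DirectionShoot component's location and rotation and plays FireCue, without aiming at the stored player.
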(event OnComponentBeginOverlap(BC_ArreaForShoot)
  (params (OverlappedComponent :type Primitive%20Component%20Object%20Reference) (OtherActor :type Actor%20Object%20Reference) (OtherComp :type Primitive%20Component%20Object%20Reference) (OtherBodyIndex :type Integer) (bFromSweep :type Boolean) (SweepResult :type Hit%20Result%20Structure%20%28by%20ref%29))
  (bind (_isplayer_ _player) (Class|BPIPlayer|BPIIsPlayer?(Message) OtherActor))
  (if _isplayer_
    (Variables|Default|SetBP_Player2D _player)
    (CallFunction|FShoot)
    (bind _returnvalue (Utilities|Time|SetTimerbyFunctionName 0 "FShoot" 1.5 true))
    (Variables|Default|SetTimer_FShoot _returnvalue)))

(event OnComponentEndOverlap(BC_ArreaForShoot)
  (params (OverlappedComponent :type Primitive%20Component%20Object%20Reference) (OtherActor :type Actor%20Object%20Reference) (OtherComp :type Primitive%20Component%20Object%20Reference) (OtherBodyIndex :type Integer))
  (bind _isplayer_ (Class|BPIPlayer|BPIIsPlayer?(Message) OtherActor))
  (if _isplayer_
    (Variables|Default|SetBP_Player2D 0)
    (Utilities|Time|ClearandInvalidateTimerbyHandle (Variables|Default|GetTimer_FShoot))))

(event EventBeginPlay)

(event Collision|EventActorBeginOverlap
  (params (OtherActor :type Actor%20Object%20Reference)))

(event EventTick
  (params (DeltaSeconds :type Float%20%28single-precision%29)))

(fn ConstructionScript)

(fn FShoot
  (bind _directionshoot (Variables|Default|GetDirectionShoot))
  (bind _returnvalue (Transformation|GetWorldTransform _directionshoot))
  (Game|SpawnActorfromClass "/Game/Chicken/Core/BP/Weapon/BP_Shoot.BP_Shoot_C" (Math|Transform|MakeTransform (.location _returnvalue) (.rotation _returnvalue)) "AlwaysSpawn" 0 0)
  (Audio|Components|Audio|Play (Variables|Default|Getfire_Cue) 0.0))