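; BP_Direction is a water-current volume that pushes the player along a set direction and can optionally deal damage.
; The construction script stretches a spline mesh between Start and Finish and aims an arrow along that line.
; Mesh overlaps, filtered through a player-check interface, store the player, toggle its Water flag and control a looping flow sound.
; A delayed Tick applies a large force along the arrow to the stored player's movement.
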(event OnComponentBeginOverlap(SplineMesh)
  (params (OverlappedComponent :type Primitive%20Component%20Object%20Reference) (OtherActor :type Actor%20Object%20Reference) (OtherComp :type Primitive%20Component%20Object%20Reference) (OtherBodyIndex :type Integer) (bFromSweep :type Boolean) (SweepResult :type Hit%20Result%20Structure%20%28by%20ref%29))
  (bind (_isplayer_ _player) (Class|BPIPlayer|BPIIsPlayer?(Message) OtherActor))
  (if _isplayer_
    (bind _output_get (Variables|Default|Setplayer _player))
    (Variables|/Game/Chicken/Core/BP_Characters/BP_Player/Level/BP_Player2D.BP_Player2D_C|SetbWater? _output_get true)
    (Audio|Components|Audio|Play (Variables|Default|GetFlowWater_Cue) 0.0)))

(event OnComponentEndOverlap(SplineMesh)
  (params (OverlappedComponent :type Primitive%20Component%20Object%20Reference) (OtherActor :type Actor%20Object%20Reference) (OtherComp :type Primitive%20Component%20Object%20Reference) (OtherBodyIndex :type Integer))
  (bind (_isplayer_ _player) (Class|BPIPlayer|BPIIsPlayer?(Message) OtherActor))
  (if _isplayer_
    (Variables|/Game/Chicken/Core/BP_Characters/BP_Player/Level/BP_Player2D.BP_Player2D_C|SetbWater? _player false)
    (Variables|Default|Setplayer 0)
    (Audio|Components|Audio|Stop (Variables|Default|GetFlowWater_Cue))))

(event OnAudioFinished(FlowWater_Cue)
  (Variables|Default|Getplayer
    (:then
      (Audio|Components|Audio|Play (Variables|Default|GetFlowWater_Cue) 0.0))
    (:else)))

(event EventTick
  (params (DeltaSeconds :type Float%20%28single-precision%29))
  (Utilities|FlowControl|Delay 0.1)
  (bind _player (Variables|Default|Getplayer)
    (:then
      (bind _charactermovement (Variables|/Script/Engine.Character|GetCharacterMovement _player)
        (:then
          (Physics|AddForce _charactermovement (* (Math|Vector|GetForwardVector (Variables|Default|GetArrow)) 1e+07))
          (if (Variables|Default|GetDamage?)
            (Game|Damage|ApplyPointDamage _player 1.0 (Math|Vector|MakeVector 0.0 0.0 0.0) (Collision|MakeHitResult false false 0.0 0.0 "0, 0, 0" "0, 0, 0" "0,0,1" "0,0,1" 0 0))))
        (:else)))
    (:else)))

(fn ConstructionScript
  (bind _spline (Variables|Default|GetSpline))
  (Spline|SetLocationatSplinePoint _spline 0 (Variables|Default|GetStart) "Local" true)
  (Spline|SetLocationatSplinePoint _spline 1 (Variables|Default|GetFinish) "Local" true)
  (SplineMesh|SetStartandEnd (Variables|Default|GetSplineMesh) (Variables|Default|GetStart) (Spline|GetTangentatSplinePoint _spline 0 "Local") (Variables|Default|GetFinish) (Spline|GetTangentatSplinePoint _spline 1 "Local") true :!class /Script/Engine.SplineMeshComponent)
  (Transformation|SetRelativeRotation (Variables|Default|GetArrow) (Math|Rotator|FindLookatRotation (Variables|Default|GetStart) (Variables|Default|GetFinish)) false false))