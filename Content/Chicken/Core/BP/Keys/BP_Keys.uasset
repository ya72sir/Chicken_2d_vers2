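; BP_Keys is a collectible key pickup with a Paper2D sprite, identified by an enum.
; Its construction script pins the actor to Y=0, then loads the key's data table row to set the sprite, printing a warning if none exists.
; On box overlap by a player, it uses interface calls to add the key and show a named message with its sprite.
; It then plays a sound, hides and destroys itself after a short delay.
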(event OnComponentBeginOverlap(Box)
  (params (OverlappedComponent :type Primitive%20Component%20Object%20Reference) (OtherActor :type Actor%20Object%20Reference) (OtherComp :type Primitive%20Component%20Object%20Reference) (OtherBodyIndex :type Integer) (bFromSweep :type Boolean) (SweepResult :type Hit%20Result%20Structure%20%28by%20ref%29))
  (bind _infokey (Variables|Private_ParamKey|GetInfoKey))
  (bind (_id _name _ps_key) (Utilities|Struct|BreakStr_Key _infokey))
  (bind (_isplayer_ _player) (Class|BPIPlayer|BPIIsPlayer?(Message) OtherActor))
  (if _isplayer_
    (Default|BPIAddKey _player (Variables|Default|GetEnum_NameKey))
    (Default|BPIShowMessage _player (Utilities|Text|FormatText "You found the key - {NameKey}" (Utilities|Text|ToText(String) _name)) _ps_key)
    (Audio|Components|Audio|Play (Variables|Default|GetTakeMoney_Cue) 0.0)
    (Rendering|SetActorHiddenInGame self true)
    (Utilities|FlowControl|Delay 0.5)
    (Actor|DestroyActor)))

(fn ConstructionScript
  (bind _returnvalue (Transformation|GetActorLocation))
  (bind _enum_namekey (Variables|Default|GetEnum_NameKey))
  (bind (_isvalid_ _out_row) (CallFunction|BFLGetDataTableKey _enum_namekey))
  (Transformation|SetActorLocation (Math|Vector|MakeVector (.x _returnvalue) 0.0 (.z _returnvalue)) false false)
  (if _isvalid_
    (bind _output_get (Variables|Private_ParamKey|SetInfoKey _out_row))
    (Rendering|Components|Sprite|SetSprite (Variables|Default|GetCompPS_Key) (.PS_Key (Utilities|Struct|BreakStr_Key _output_get)))
    (else
      (Development|PrintString "NopeKey"))))