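; BP_Elevator is a level actor whose Paper2D sprite travels back and forth along a spline.
; The construction script applies the chosen sprite and rebuilds the spline from the PointsVector array.
; Each Tick, FMoveElevator advances or reduces a distance by delta time times Speed, reversing direction at either end.
; It places the sprite at that distance in local space, then snaps it to the closest world-space spline point.
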(event EventTick
  (params (DeltaSeconds :type Float%20%28single-precision%29))
  (CallFunction|FMoveElevator DeltaSeconds))

(fn ConstructionScript
  (bind _sprite (Variables|Default|GetSprite))
  (Utilities|IsValid _sprite
    (:Is%20Valid
      (Rendering|Components|Sprite|SetSprite (Variables|Default|GetPaperSprite) _sprite))
    (:Is%20Not%20Valid
      _))
  (Spline|ClearSplinePoints (Variables|Default|GetSpline) true)
  (for (_array_element _array_index) (Variables|Default|GetpointsVector)
    (Class|SplineComponent|AddPoint (Variables|Default|GetSpline) (Utilities|Struct|MakeSplinePoint (Math|Conversions|ToFloat(Integer) _array_index) _array_element "0.000000,0.000000,0.000000" "0.000000,0.000000,0.000000" "0.000000,0.000000,0.000000" "1.000000,1.000000,1.000000" "Curve") true)))

(fn FMoveElevator
  (params (tick :type Float%20%28single-precision%29))
  (bind _papersprite (Variables|Default|GetPaperSprite))
  (LocalVariables|SetLSpeed (* tick (Variables|Default|Getspeed)))
  (if (Variables|Default|GetMoveUp?)
    (if (>= (Variables|Default|GetuseLength) (Spline|GetSplineLength (Variables|Default|GetSpline)))
      (Variables|Default|SetMoveUp? false)
      (else
        (Variables|Default|SetuseLength (+ (Variables|Default|GetuseLength) (LocalVariables|GetLSpeed)))
        (Transformation|SetRelativeLocation _papersprite (Spline|GetLocationatDistanceAlongSpline (Variables|Default|GetSpline) (Variables|Default|GetuseLength) "Local") false false :!label _label)
        (Transformation|SetWorldLocation (Variables|Default|GetPaperSprite) (Spline|FindLocationClosesttoWorldLocation (Variables|Default|GetSpline) (Transformation|GetWorldLocation _papersprite) "World") false false)))
    (elif (<= (Variables|Default|GetuseLength) 0.0)
      (Variables|Default|SetMoveUp? true)
      (else
        (Variables|Default|SetuseLength (- (Variables|Default|GetuseLength) (LocalVariables|GetLSpeed)))
        (goto _label)))))