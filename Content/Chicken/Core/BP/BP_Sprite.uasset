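; BP_Sprite is a construction-time builder for a horizontal strip of Paper2D sprites with start, repeated fill and end pieces.
; The construction script snaps Y to Layer, applies Scale, and derives the fill count from HotizontEndPoint's length and the start sprite's width.
; When EnabledCollision is set, it adds a box spanning the strip, aims RotationHelper toward the end point and applies the optional Flip rotation.
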(event EventBeginPlay)

(event Collision|EventActorBeginOverlap
  (params (OtherActor :type Actor%20Object%20Reference)))

(event EventTick
  (params (DeltaSeconds :type Float%20%28single-precision%29)))

(fn ConstructionScript
  (bind _returnvalue (Transformation|GetActorLocation))
  (bind _returnvalue_2 (Transformation|GetActorLocation))
  (bind (_x _y _z) (Math|Vector|BreakVector _returnvalue_2))
  (Transformation|SetActorLocation (Math|Vector|MakeVector _x (Math|Conversions|ToFloat(Integer) (Variables|Default|GetLayer)) _z) false false)
  (Transformation|SetWorldScale3D (Variables|Default|GetFirstSprite) (Math|Conversions|ToVector(Float) (Variables|Default|GetScale)))
  (Rendering|Components|Sprite|SetSprite (Variables|Default|GetFirstSprite) (Variables|Sprite|GetStartSprite))
  (Rendering|Components|Sprite|SetSprite (Variables|Default|GetLastSprite) (Variables|Sprite|GetEndSprite))
  (Transformation|SetRelativeLocation (Variables|Default|GetFirstSprite) "0, 0, 0" false false)
  (Variables|Default|SetSpriteWidth (* 2 (.X (Math|Vector|BreakVector (.BoxExtent (Collision|GetComponentBounds (Variables|Default|GetFirstSprite)))))))
  (Variables|Default|SetLoops (- (Math|Float|Floor (/ (Math|Vector|VectorLength (Variables|Default|GetHotizont_EndPoint)) (Variables|Default|GetSpriteWidth))) 1))
  (for _index (range 1 (Variables|Default|GetLoops))
    (bind _returnvalue_3 (AddComponent|AddPaperSpriteComponent false))
    (Class|SceneComponent|Attachto _returnvalue_3 (Variables|Default|GetFirstSprite) "None" "KeepRelativeOffset" true)
    (Transformation|SetRelativeLocation _returnvalue_3 (Math|Vector|MakeVector (* _index (/ (Variables|Default|GetSpriteWidth) (Variables|Default|GetScale))) 0.0 0.0) false false)
    (Rendering|Components|Sprite|SetSprite _returnvalue_3 (Variables|Sprite|GetFillSprite)))
  (Transformation|SetRelativeLocation (Variables|Default|GetLastSprite) (Math|Vector|MakeVector (+ (* (Variables|Default|GetLoops) (/ (Variables|Default|GetSpriteWidth) (Variables|Default|GetScale))) (/ (Variables|Default|GetSpriteWidth) (Variables|Default|GetScale))) 0.0 0.0) false false)
  (if (Variables|Default|GetEnabledCollision?)
    (bind _returnvalue_4 (AddComponent|AddBoxComponent true))
    (Variables|Default|SetboxCollision _returnvalue_4)
    (Components|Box|SetBoxExtent (Variables|Default|GetboxCollision) (/ (Math|Vector|MakeVector (* (+ (Variables|Default|GetLoops) 2) (Variables|Default|GetSpriteWidth)) (Variables|Default|GetSpriteWidth) (Variables|Default|GetSpriteWidth)) 2.0) true)
    (Class|SceneComponent|Attachto (Variables|Default|GetboxCollision) (Variables|Default|GetFirstSprite) "None" "SnapToTarget" true)
    (Transformation|SetRelativeLocation (Variables|Default|GetboxCollision) (Math|Vector|MakeVector (/ (* (+ (Variables|Default|GetLoops) 1) (/ (Variables|Default|GetSpriteWidth) (Variables|Default|GetScale))) 2.0) 0.0 0.0) false false)
    (Transformation|SetWorldRotation (Variables|Default|GetRotationHelper) (Math|Rotator|FindLookatRotation _returnvalue (+ _returnvalue (Variables|Default|GetHotizont_EndPoint))) false false)
    (Transformation|AddLocalRotation (Variables|Default|GetFirstSprite) (Math|Rotator|SelectRotator "0, 0,180.000000" "0, 0, 0" (Variables|Default|GetFlip)) false false)))