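; BP_FlyNPC is a Paper2D info NPC that offers dialog and quest interaction when the player overlaps its sphere.
; A looping timer with a randomized period flips the sprite's facing, while a timeline rotates its marker.
; Overlap calls the GameMode's quest-attack dialog if its injected quest ID matches the completed one, otherwise the HUD dialog.
; Disabling the quest hides the marker, returns the quest ID and destroys the actor shortly after.
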(event Custom|Ev_RandomRotation
  (bind _isa (Utilities|FlowControl|FlipFlop)
    (:A
      _)
    (:B
      _))
  (Transformation|SetRelativeRotation (Variables|Default|GetPaperFlipbook_NPC) (select _isa "0,-180.000000, 0" "0, 0, 0") false false))

(event Custom|Ev_DestoyActor
  (Utilities|FlowControl|Delay 0.05)
  (Actor|DestroyActor))

(event EventBeginPlay
  (Utilities|Time|SetTimerbyEvent (delegate Custom|Ev_RandomRotation) (Math|Random|RandomFloatinRange 1.0 5.0) true)
  (bind _newtrack_0 (Timeline|Timeline_Rotation Play)
    (:Update
      (Transformation|SetRelativeRotation (Variables|Default|GetPaperFlipbook_Mark) (Math|Rotator|MakeRotator 0.0 _newtrack_0 0.0) false false))))

(event OnComponentBeginOverlap(SphColl_Interaction)
  (params (OverlappedComponent :type Primitive%20Component%20Object%20Reference) (OtherActor :type Actor%20Object%20Reference) (OtherComp :type Primitive%20Component%20Object%20Reference) (OtherBodyIndex :type Integer) (bFromSweep :type Boolean) (SweepResult :type Hit%20Result%20Structure%20%28by%20ref%29))
  (bind _isplayer_ (Class|BPIPlayer|BPIIsPlayer?(Message) OtherActor))
  (if _isplayer_
    (if (== (Variables|/Game/Chicken/Core/BP_Characters/BP_Player/Level/BP_GM_Player2DLevel.BP_GM_Player2DLevel_C|GetQuest_CompletedID (CallFunction|BFLGetGameModeBP)) (Variables|Default|GetQuest_ID))
      (Default|EvShowDialogQuestAttack (CallFunction|BFLGetGameModeBP) self)
      (else
        (Default|EvWBPDialog (CallFunction|BFLGetHUD) self)))))

(event EventBPINPCSetIdDialogandSetIdQuest
  (params (ID%20For%20Dialog%20System :type Integer) (ID%20For%20Quest%20System :type Integer))
  (Variables|Default|SetDialog_ID ID%20For%20Dialog%20System)
  (Variables|Default|SetQuest_ID ID%20For%20Quest%20System))

(fn ConstructionScript)

(fn BPINPCDisableQuest
  (CallFunction|EvDestoyActor)
  (Rendering|SetVisibility (Variables|Default|GetPaperFlipbook_Mark) false false)
  (return (Variables|Default|GetQuest_ID)))

(fn BPINPCIsDead?
  (return false false))