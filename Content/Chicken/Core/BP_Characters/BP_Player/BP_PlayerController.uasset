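; Player controller that routes input to the player character and forwards menu, pause, quest, dialog and level-flow events to the HUD and game mode.
; Movement and jump depend on the HUD's current widget action and a movement lock; jump also closes finished dialogs or stops go-to-camera.
; Movement input triggers game over when the character is invalid.
; It also plays Enter-skippable cutscenes that start the game when ended, and Z completes the level.
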(event Custom|Ev_PlaySkippableCutscene
  (params (SequencePlayer :type Movie%20Scene%20Sequence%20Player%20Object%20Reference))
  (bind _output_get (Variables|Private/Params|SetSequencePlayer SequencePlayer))
  (Sequencer|Player|Play _output_get :!class /Script/MovieScene.MovieSceneSequencePlayer)
  (EventDispatchers|BindEventtoOnFinished _output_get (delegate Custom|Ev_StopPlayingSkippableCutscene))
  (Default|EvCreateHUD (CallFunction|BFLGetHUD))
  (bind _returnvalue (UserInterface|CreateWidget "/Game/Chicken/Core/BP_Widgets/Interface/WBP_SkipIntro.WBP_SkipIntro_C" self))
  (UserInterface|Viewport|AddtoViewport _returnvalue 0))

(event Custom|Ev_StopPlayingSkippableCutscene
  (Utilities|FlowControl|DoOnce false
    (:Completed
      (bind _sequenceplayer (Variables|Private/Params|GetSequencePlayer)
        (:then
          (Sequencer|Player|Stop _sequenceplayer :!class /Script/MovieScene.MovieSceneSequencePlayer))
        (:else
          _))
      (Default|EvCreateHUD (CallFunction|BFLGetHUD))
      (Default|EvStartGame (CallFunction|BFLGetGameModeBP))
      (Utilities|IsValid (stale Custom|Ev_PlaySkippableCutscene _returnvalue)
        (:Is%20Valid
          (Widget|RemovefromParent (stale Custom|Ev_PlaySkippableCutscene _returnvalue)))))))

(event Custom|Ev_SetBPPlayerState
  (params (BP_PlayerState :type BP%20Player%20State%20Object%20Reference))
  (Variables|Default|SetBP_PlayerState BP_PlayerState))

(event Custom|Ev_ExitPauseMenu
  (Default|EvMenu (CallFunction|BFLGetHUD)))

(event EventPossess
  (params (PossessedPawn :type Pawn%20Object%20Reference))
  (Utilities|FlowControl|DoOnce false
    (:Completed
      (bind (_isplayer_ _player) (Class|BPIPlayer|BPIIsPlayer?(Message) PossessedPawn))
      (if _isplayer_
        (Variables|Private/Params|SetBP_Player2D _player)))))

(event Input|ActionEvents|InputActionAct_Menu
  (params (Key :type Key%20Structure :default "None"))
  (:Pressed
    (CallFunction|EvExitPauseMenu)))

(event Input|ActionEvents|InputActionAct_Pause
  (params (Key :type Key%20Structure :default "None"))
  (:Pressed
    (Default|EvPause (CallFunction|BFLGetHUD))))

(event Input|ActionEvents|InputActionAct_QuestMessage
  (params (Key :type Key%20Structure :default "None"))
  (:Pressed
    (bind _wbp_hud (Variables|/Game/Chicken/Core/BP_Characters/BP_Player/Level/BP_HUD.BP_HUD_C|GetWBP_HUD (CallFunction|BFLGetHUD))
      (:then
        (Default|EvShowMessageQuest _wbp_hud))
      (:else
        (Development|PrintString "Error HUD" true true "(R=1.000000,G=0.130655,B=0.000000,A=1.000000)")))))

(event Input|KeyboardEvents|Enter
  (params (Key :type Key%20Structure :default "None"))
  (:Pressed
    (Utilities|FlowControl|DoOnce false
      (:Completed
        (bind _sequenceplayer (Variables|Private/Params|GetSequencePlayer)
          (:then
            (Sequencer|Player|Stop _sequenceplayer :!class /Script/MovieScene.MovieSceneSequencePlayer))
          (:else
            _))
        (Default|EvCreateHUD (CallFunction|BFLGetHUD))
        (Default|EvStartGame (CallFunction|BFLGetGameModeBP))
        (Utilities|IsValid (stale Custom|Ev_PlaySkippableCutscene _returnvalue)
          (:Is%20Valid
            (Widget|RemovefromParent (stale Custom|Ev_PlaySkippableCutscene _returnvalue))))))))

(event Input|KeyboardEvents|Z
  (params (Key :type Key%20Structure :default "None"))
  (:Pressed
    (CallFunction|EvLevelComplited)))

(event Custom|Ev_DisableMoveCharacter
  (params (DisableMove? :type Boolean))
  (bind _output_get (Variables|Private/Params|SetDisableMove? DisableMove?))
  (if _output_get
    (Components|Movement|StopMovementImmediately (Variables|/Script/Engine.Character|GetCharacterMovement (CallFunction|BFLGetPlayerCharacterBP)))
    (Input|DisableInput (CallFunction|BFLGetPlayerCharacterBP) (CallFunction|BFLGetPlayerControllerBP))
    (else
      (Input|EnableInput (CallFunction|BFLGetPlayerCharacterBP) (CallFunction|BFLGetPlayerControllerBP)))))

(event Custom|Ev_DialogOpen
  (params (WBP_Dialog :type WBP%20Dialog%20Object%20Reference))
  (bind _output_get (Variables|WBP|SetWBP_Dialog WBP_Dialog))
  (Input|SetInputModeGameandUI (CallFunction|BFLGetPlayerControllerBP) _output_get "LockAlways" true))

(event Custom|Ev_GoToCamera
  (params (bGoToCamera? :type Boolean))
  (Variables|Private/Params|SetGoToCamera? bGoToCamera?))

(event Input|ActionEvents|InputActionAct_Jump_ExitDialogWidget
  (params (Key :type Key%20Structure))
  (:Pressed
    (switch Utilities|FlowControl|Switch|SwitchonEWBPPlayerController (Variables|/Game/Chicken/Core/BP_Characters/BP_Player/Level/BP_HUD.BP_HUD_C|GetWBP_CurrentAction (CallFunction|BFLGetHUD))
      (:NewEnumerator0
        (if (not (Game|IsGamePaused))
          (if (Variables|Private/Params|GetDisableMove?)
            (if (Variables|Private/Params|GetGoToCamera?)
              (Default|EvStopGotoCamera (CallFunction|BFLGetPlayerCharacterBP))
              (Variables|Private/Params|SetGoToCamera? false))
            (else
              (Default|EvJump (CallFunction|BFLGetPlayerCharacterBP))))))
      (:NewEnumerator2
        (if (Variables|/Game/Chicken/Core/BP_Widgets/HUD/Dialog/WBP_Dialog.WBP_Dialog_C|GetDialogClose? (Variables|WBP|GetWBP_Dialog))
          (bind _ownerdialogsys (Variables|/Game/Chicken/Core/BP_Widgets/HUD/Dialog/WBP_Dialog.WBP_Dialog_C|GetOwnerDialogSys (Variables|WBP|GetWBP_Dialog))
            (:then
              (Class|BPINPC|BPINPCDisableQuest(Message) _ownerdialogsys))
            (:else
              _))
          (CallFunction|EvExitCurrentWidget)
          (CallFunction|EvDisableMoveCharacter false)
          (Default|EvDisableQuest (CallFunction|BFLGetGameModeBP)))))))

(event Custom|Ev_WBPDialog
  (params (OwnerDialogSys :type Actor%20Object%20Reference))
  (Default|EvWBPDialog (CallFunction|BFLGetHUD) OwnerDialogSys))

(event Custom|Ev_WBPPauseGame
  (Default|EvWBPPauseGame (CallFunction|BFLGetHUD)))

(event Custom|Ev_WBPMenu
  (Default|EvWBPMenu (CallFunction|BFLGetHUD)))

(event Custom|Ev_ShowCurrentWBP
  (Default|EvShowCurrentWBP (CallFunction|BFLGetHUD)))

(event Custom|Ev_ExitCurrentWidget
  (Default|EvExitMenuorPause (CallFunction|BFLGetHUD)))

(event Custom|Ev_LevelComplited
  (Default|EvLevelComplited (CallFunction|BFLGetGameModeBP)))

(event Custom|Ev_SelectLevels
  (Default|EvSelectLevels (CallFunction|BFLGetHUD)))

(event Custom|Ev_WBPFinishGame
  (Default|EvWBPFinishGame (CallFunction|BFLGetHUD)))

(event Custom|Ev_BackMenu
  (Default|EvCloseLevelGotoMenu (CallFunction|BFLGetHUD)))

(fn ConstructionScript)

(fn FGetBPPlayer2D
  (return (Variables|Private/Params|GetBP_Player2D)))

(event Input|AxisEvents|InputAxisMoveForward
  (params (AxisValue :type Float%20%28single-precision%29))
  (bind _asgm_player_2dlevel (CallFunction|BFLGetGameModeBP))
  (bind _bp_player2d (CallFunction|BFLGetPlayerCharacterBP))
  (Utilities|MCurrentAction
    (:_None
      (if (Game|IsGamePaused)
        (if (!= AxisValue 0.0)
          (if (Variables|Private/Params|GetGamepadIsActive?)
            _))
        (elif (not (Variables|Private/Params|GetDisableMove?))
          (Utilities|IsValid _bp_player2d
            (:Is%20Valid
              (Default|EvMoveForward _bp_player2d AxisValue))
            (:Is%20Not%20Valid
              (Utilities|IsValid _asgm_player_2dlevel
                (:Is%20Valid
                  (Default|EvGameOver _asgm_player_2dlevel))))))))))

(event Input|AxisEvents|InputAxisMoveRight
  (params (AxisValue :type Float%20%28single-precision%29))
  (bind _asgm_player_2dlevel (CallFunction|BFLGetGameModeBP))
  (bind _bp_player2d (CallFunction|BFLGetPlayerCharacterBP))
  (Utilities|MCurrentAction
    (:_None
      (if (Game|IsGamePaused)
        (if (!= AxisValue 0.0)
          (if (Variables|Private/Params|GetGamepadIsActive?)
            _))
        (elif (not (Variables|Private/Params|GetDisableMove?))
          (Utilities|IsValid _bp_player2d
            (:Is%20Valid
              (Default|EvMoveRight _bp_player2d AxisValue))
            (:Is%20Not%20Valid
              (Utilities|IsValid _asgm_player_2dlevel
                (:Is%20Valid
                  (Default|EvGameOver _asgm_player_2dlevel))))))))))

(event Input|ActionEvents|InputActionAct_AnyKey
  (params (Key :type Key%20Structure :default "None"))
  (:Pressed
    (Default|EvAnyKeys (CallFunction|BFLGetHUD) Key)))

(event EventBeginPlay
  (bind _asbp_game_instance (CallFunction|BFLGetGameInstanceBP))
  (Utilities|IsValid _asbp_game_instance
    (:Is%20Valid
      (Default|EvInit _asbp_game_instance)
      (CallFunction|BFLShowMouseCursor false)
      (if (Utilities|Enum|NotEqual(Enum) (Default|FGetCurrentLevel (CallFunction|BFLGetGameInstanceBP)) "NewEnumerator0")
        (Default|EvStartGame (CallFunction|BFLGetGameModeBP))))))