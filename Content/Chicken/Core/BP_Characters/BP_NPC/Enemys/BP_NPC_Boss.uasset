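; BP_NPC_Boss is the boss enemy NPC Blueprint, displayed through a Paper2D flipbook component.
; EvSetPaperFlipbook applies the current flipbook to PFBoss when flipbook updates are enabled.
; EvMove computes a per-tick movement delta from speed when movement is enabled, but does not apply it here.
; BeginPlay, overlap, Tick and the construction script are empty, and nothing in this Blueprint calls either custom event.
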(event EventBeginPlay)

(event Collision|EventActorBeginOverlap
  (params (OtherActor :type Actor%20Object%20Reference)))

(event EventTick
  (params (DeltaSeconds :type Float%20%28single-precision%29)))

(event Custom|EvSetPaperFlipbook
  (if (Variables|Param/Flipbook|GetEnbaledPaperFlipbook?)
    (Sprite|SetFlipbook (Variables|Default|GetPF_Boss) (Variables|Param/Flipbook|GetFlipbook))))

(event Custom|EvMove
  (params (Tick :type Float%20%28single-precision%29))
  (if (Variables|Param/Move|GetEnabledMove?)
    (Variables|Private|SetDeltaForMove (* Tick (Variables|Param/Move|GetSpeed)))))

(fn ConstructionScript)