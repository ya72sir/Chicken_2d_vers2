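; BP_FlowWater is a level-placed water stretch that flags players as being in water while they overlap it.
; The construction script places two spline points at the Start and Finish variables, then stretches the spline mesh between them using the spline's tangents, read in world space.
; Spline mesh overlap events identify players through a Blueprint interface message and toggle their BWater flag on enter and exit.
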(event OnComponentBeginOverlap(SplineMesh)
  (params (OverlappedComponent :type Primitive%20Component%20Object%20Reference) (OtherActor :type Actor%20Object%20Reference) (OtherComp :type Primitive%20Component%20Object%20Reference) (OtherBodyIndex :type Integer) (bFromSweep :type Boolean) (SweepResult :type Hit%20Result%20Structure%20%28by%20ref%29))
  (bind (_isplayer_ _player) (Class|BPIPlayer|BPIIsPlayer?(Message) OtherActor))
  (if _isplayer_
    (Variables|/Game/Chicken/Core/BP_Characters/BP_Player/Level/BP_Player2D.BP_Player2D_C|SetBWater? _player true)))

(event OnComponentEndOverlap(SplineMesh)
  (params (OverlappedComponent :type Primitive%20Component%20Object%20Reference) (OtherActor :type Actor%20Object%20Reference) (OtherComp :type Primitive%20Component%20Object%20Reference) (OtherBodyIndex :type Integer))
  (bind (_isplayer_ _player) (Class|BPIPlayer|BPIIsPlayer?(Message) OtherActor))
  (if _isplayer_
    (Variables|/Game/Chicken/Core/BP_Characters/BP_Player/Level/BP_Player2D.BP_Player2D_C|SetBWater? _player false)))

(fn ConstructionScript
  (bind _spline (Variables|Default|GetSpline))
  (Spline|SetLocationatSplinePoint _spline 0 (Variables|Default|GetStart) "Local" true)
  (Spline|SetLocationatSplinePoint _spline 1 (Variables|Default|GetFinish) "Local" true)
  (SplineMesh|SetStartandEnd (Variables|Default|GetSplineMesh) (Variables|Default|GetStart) (Spline|GetTangentatSplinePoint _spline 0 "World") (Variables|Default|GetFinish) (Spline|GetTangentatSplinePoint _spline 1 "World") true :!class /Script/Engine.SplineMeshComponent))