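; Blueprint function library for the 2D player game, giving global typed access to the game's core framework objects.
; Getters return the cast game mode, controller, 2D character, game instance, game state, player state and HUD.
; The controller getter prefers the game mode's stored reference, falls back to player index 0, and feeds several other functions.
; Helpers also look up DT_Keys rows by enum name and toggle mouse cursor and input mode around a focus widget.
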(fn BFLGetGameModeBP
  (bind _asbp_gm_player_2dlevel (Utilities|Casting|CastToBP_GM_Player2DLevel (Game|GetGameMode))
    (:then
      _)
    (:CastFailed
      _))
  (return _asbp_gm_player_2dlevel))

(fn BFLGetPlayerControllerBP
  (bind _asgm_player_2dlevel (CallFunction|BFLGetGameModeBP))
  (Utilities|IsValid _asgm_player_2dlevel
    (:Is%20Valid
      (Variables|/Game/Chicken/Core/BP_Characters/BP_Player/Level/BP_GM_Player2DLevel.BP_GM_Player2DLevel_C|GetBP_PlayerController _asgm_player_2dlevel
        (:then
          (return (Variables|/Game/Chicken/Core/BP_Characters/BP_Player/Level/BP_GM_Player2DLevel.BP_GM_Player2DLevel_C|GetBP_PlayerController (CallFunction|BFLGetGameModeBP))))
        (:else
          _)))
    (:Is%20Not%20Valid
      _))
  (bind _asbp_player_controller (Utilities|Casting|CastToBP_PlayerController (Game|GetPlayerController 0)))
  (return _asbp_player_controller))

(fn BFLGetPlayerCharacterBP
  (bind _asbp_player_controller (CallFunction|BFLGetPlayerControllerBP))
  (bind _bp_player2d (Default|FGetBPPlayer2D _asbp_player_controller))
  (Utilities|IsValid _bp_player2d
    (:Is%20Valid
      (return _bp_player2d))
    (:Is%20Not%20Valid
      (return 0))))

(fn BFLGetDataTableKey
  (params (NameKey :type ENameKey%20Enum :default "NewEnumerator0"))
  (bind _returnvalue (Utilities|GetDataTableRow "/Game/Chicken/Core/DataTable/DT_Keys.DT_Keys" (Utilities|String|StringToName (Utilities|String|EnumtoString NameKey)))
    (:then
      (return true _returnvalue))
    (:RowNotFound
      (return false ""))))

(fn BFLGetGameInstanceBP
  (bind _asbp_game_instance (Utilities|Casting|CastToBP_GameInstance (Game|GetGameInstance))
    (:then
      _)
    (:CastFailed
      _))
  (return _asbp_game_instance))

(fn BFLShowMouseCursor
  (params (Enabled :type Boolean) (InWidgetToFocus :type Widget%20Object%20Reference))
  (bind _asbp_player_controller (CallFunction|BFLGetPlayerControllerBP))
  (Utilities|IsValid _asbp_player_controller
    (:Is%20Valid
      (bind _output_get (Variables|/Script/Engine.PlayerController|SetbShowMouseCursor _asbp_player_controller (and Enabled (Utilities|IsValid InWidgetToFocus))))
      (if _output_get
        (Input|SetInputModeGameandUI (CallFunction|BFLGetPlayerControllerBP) InWidgetToFocus "LockAlways" true :!label _label)
        (else
          (Utilities|IsValid InWidgetToFocus
            (:Is%20Valid
              (goto _label))
            (:Is%20Not%20Valid
              (Input|SetInputModeGameOnly (CallFunction|BFLGetPlayerControllerBP)))))))))

(fn BFLGetGameState
  (bind _asbp_game_state (Utilities|Casting|CastToBP_GameState (Game|GetGameState))
    (:then
      _)
    (:CastFailed
      _))
  (return _asbp_game_state))

(fn BFLGetPlayerState
  (Utilities|IsValid (CallFunction|BFLGetPlayerControllerBP)
    (:Is%20Valid
      (Utilities|IsValid (Variables|/Script/Engine.Controller|GetPlayerState (CallFunction|BFLGetPlayerControllerBP))
        (:Is%20Valid
          (bind _asbp_player_state (Utilities|Casting|CastToBP_PlayerState (Variables|/Script/Engine.Controller|GetPlayerState (CallFunction|BFLGetPlayerControllerBP)))
            (:then
              (return _asbp_player_state))
            (:CastFailed
              (return 0))))
        (:Is%20Not%20Valid
          _)))
    (:Is%20Not%20Valid
      _))
  (return 0))

(fn BFLGetHUD
  (bind _asbp_hud (Utilities|Casting|CastToBP_HUD (HUD|GetHUD (CallFunction|BFLGetPlayerControllerBP)))
    (:then
      (return _asbp_hud))
    (:CastFailed
      (return 0))))