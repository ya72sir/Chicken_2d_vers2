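; BP_AddLife is a health pickup for a level, shown as a Paper2D sprite set in the construction script.
; A timeline started on BeginPlay drives the sprite's yaw rotation.
; On sprite overlap, Blueprint interface messages check for the player and try to add AddLife.
; Success shows a health-restored message and destroys the pickup; failure reports that health is already full and leaves it in place.
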(event OnComponentBeginOverlap(PaperSprite)
  (params (OverlappedComponent :type Primitive%20Component%20Object%20Reference) (OtherActor :type Actor%20Object%20Reference) (OtherComp :type Primitive%20Component%20Object%20Reference) (OtherBodyIndex :type Integer) (bFromSweep :type Boolean) (SweepResult :type Hit%20Result%20Structure%20%28by%20ref%29))
  (bind (_isplayer_ _player) (Class|BPIPlayer|BPIIsPlayer?(Message) OtherActor))
  (if _isplayer_
    (bind _ok_ (Class|BPIPlayer|BPIAddLife(Message) _player (Variables|Default|GetAddLife)))
    (if _ok_
      (Default|BPIShowMessage _player (Variables|Default|GetHealth%20restored) (Variables|Default|GetPS_Box))
      (Actor|DestroyActor)
      (else
        (Default|BPIShowMessage _player (Variables|Default|GetYour%20health%20is%20complete) (Variables|Default|GetPS_Box) (Variables|Default|GetSizeSprite))))))

(event EventBeginPlay
  (bind _newtrack_0 (Timeline|timeLine Play)
    (:Update
      (Transformation|SetRelativeRotation (Variables|Default|GetPaperSprite) (Math|Rotator|Lerp(Rotator) "0, 0, 0" "360.000000, 0, 0" _newtrack_0) false false))))

(fn ConstructionScript
  (Rendering|Components|Sprite|SetSprite (Variables|Default|GetPaperSprite) (Variables|Default|GetPS_Box)))