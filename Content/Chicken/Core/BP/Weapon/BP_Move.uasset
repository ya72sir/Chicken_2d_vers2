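; BP_Move is a moving hazard: a spinning Paper2D sprite that shuttles back and forth along a spline and applies point damage to the player on overlap.
; The construction script sets the first two spline points from StartMove and FinishMove.
; Tick rotates the sprite and calls FMove, which steps a distance along the spline and flips direction at either end.
; A player-check interface call gates damage, and the FlowStar audio replays whenever it finishes.
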(event OnComponentBeginOverlap(PaperSprite)
  (params (OverlappedComponent :type Primitive%20Component%20Object%20Reference) (OtherActor :type Actor%20Object%20Reference) (OtherComp :type Primitive%20Component%20Object%20Reference) (OtherBodyIndex :type Integer) (bFromSweep :type Boolean) (SweepResult :type Hit%20Result%20Structure%20%28by%20ref%29))
  (bind (_isplayer_ _player) (Class|BPIPlayer|BPIIsPlayer?(Message) OtherActor))
  (if _isplayer_
    (Game|Damage|ApplyPointDamage _player 1e+01 (Math|Vector|MakeVector 3.0 3.0 3.0) (Collision|MakeHitResult false false 0.0 0.0 "0, 0, 0" "0, 0, 0" "0,0,1" "0,0,1" 0 0))))

(event OnAudioFinished(FlowStar_Cue)
  (Audio|Components|Audio|Play (Variables|Default|GetFlowStar_Cue) 0.0))

(event EventTick
  (params (DeltaSeconds :type Float%20%28single-precision%29))
  (Transformation|AddLocalRotation (Variables|Default|GetPaperSprite) (Math|Vector|RotatorfromAxisandAngle "0.000000,1.000000,0.000000" (* DeltaSeconds (Variables|Default|GetRotationSpeed))) false false)
  (CallFunction|FMove (* DeltaSeconds (Variables|Default|GetSpeed))))

(fn ConstructionScript
  (bind _spline (Variables|Default|GetSpline))
  (Spline|SetLocationatSplinePoint _spline 0 (Variables|Default|GetStartMove) "Local" true)
  (Spline|SetLocationatSplinePoint _spline 1 (Variables|Default|GetFinishMove) "Local" true))

(fn FMove
  (params (Speed :type Float%20%28single-precision%29))
  (bind _papersprite (Variables|Default|GetPaperSprite))
  (LocalVariables|SetLSpeed Speed)
  (if (Variables|Default|GetMoveUp?)
    (if (>= (Variables|Default|GetUseLength) (Spline|GetSplineLength (Variables|Default|GetSpline)))
      (Variables|Default|SetMoveUp? false)
      (else
        (Variables|Default|SetUseLength (+ (Variables|Default|GetUseLength) (LocalVariables|GetLSpeed)))
        (Transformation|SetRelativeLocation _papersprite (Spline|GetLocationatDistanceAlongSpline (Variables|Default|GetSpline) (Variables|Default|GetUseLength) "Local") false false :!label _label)
        (Transformation|SetWorldLocation (Variables|Default|GetPaperSprite) (Spline|FindLocationClosesttoWorldLocation (Variables|Default|GetSpline) (Transformation|GetWorldLocation _papersprite) "World") false false)))
    (elif (<= (Variables|Default|GetUseLength) 0.0)
      (Variables|Default|SetMoveUp? true)
      (else
        (Variables|Default|SetUseLength (- (Variables|Default|GetUseLength) (LocalVariables|GetLSpeed)))
        (goto _label)))))