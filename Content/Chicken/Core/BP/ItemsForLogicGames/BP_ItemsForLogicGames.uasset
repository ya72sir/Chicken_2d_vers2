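; Pickup actor for logic-game items that hands itself to the player on sphere overlap.
; Its enum value names the row in DT_ItemsForLogicGames that fills ItemInfo and the Paper2D sprite, both at construction and BeginPlay.
; An overlapping player, identified through an interface call, receives the item and its message with sprite, then the GameMode is told to disable the quest.
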(event OnComponentBeginOverlap(Sphere)
  (params (OverlappedComponent :type Primitive%20Component%20Object%20Reference) (OtherActor :type Actor%20Object%20Reference) (OtherComp :type Primitive%20Component%20Object%20Reference) (OtherBodyIndex :type Integer) (bFromSweep :type Boolean) (SweepResult :type Hit%20Result%20Structure%20%28by%20ref%29))
  (bind _iteminfo (Variables|Default|GetItemInfo))
  (bind (_isplayer_ _player) (Class|BPIPlayer|BPIIsPlayer?(Message) OtherActor))
  (if _isplayer_
    (bind _output_get (Variables|Default|SetBP_Player _player))
    (Default|EvAddItemforLogic _output_get self)
    (Default|BPIShowMessage (Variables|Default|GetBP_Player) (.message _iteminfo) (.sprite _iteminfo) (.sizethesprite _iteminfo))
    (Default|EvDisableQuest (CallFunction|BFLGetGameModeBP))))

(event OnComponentEndOverlap(Sphere)
  (params (OverlappedComponent :type Primitive%20Component%20Object%20Reference) (OtherActor :type Actor%20Object%20Reference) (OtherComp :type Primitive%20Component%20Object%20Reference) (OtherBodyIndex :type Integer))
  (bind _isplayer_ (Class|BPIPlayer|BPIIsPlayer?(Message) OtherActor))
  (if _isplayer_
    (Variables|Default|SetBP_Player 0)))

(event EventBeginPlay
  (Utilities|MSetData))

(fn ConstructionScript
  (Utilities|MSetData))