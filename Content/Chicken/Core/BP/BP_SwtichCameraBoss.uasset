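; Boss-area trigger actor that switches the player's view to a level camera and opens the boss's attack quest dialog.
; The first player overlap of its box caches the player and makes the camera the view target.
; A timeline then lerps that camera from the player's side-view camera transform to its original transform, creating a manual blend.
; When it finishes, the game mode shows the dialog for the referenced boss.
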(event OnComponentBeginOverlap(Box)
  (params (OverlappedComponent :type Primitive%20Component%20Object%20Reference) (OtherActor :type Actor%20Object%20Reference) (OtherComp :type Primitive%20Component%20Object%20Reference) (OtherBodyIndex :type Integer) (bFromSweep :type Boolean) (SweepResult :type Hit%20Result%20Structure%20%28by%20ref%29))
  (bind (_isplayer_ _player) (Class|BPIPlayer|BPIIsPlayer?(Message) OtherActor))
  (if _isplayer_
    (Variables|Default|Getplayer
      (:then)
      (:else
        (Variables|Default|Setplayer _player)
        (Variables|Default|SetA (Transformation|GetWorldTransform (Variables|/Game/Chicken/Core/BP_Characters/BP_Player/Level/BP_Player2D.BP_Player2D_C|GetSideViewCameraComponent (Variables|Default|Getplayer))))
        (Game|Player|SetViewTargetwithBlend (CallFunction|BFLGetPlayerControllerBP) (Variables|Default|GetCamera) 0.0 "VTBlend_Linear" 0.0 false)
        (Variables|Default|SetB (Transformation|GetActorTransform (Variables|Default|GetCamera)))
        (bind _newtrack_0 (Timeline|Timeline_0 PlayFromStart)
          (:Update
            (Transformation|SetWorldTransform (Variables|/Script/Engine.Actor|GetRootComponent (Variables|Default|GetCamera)) (Math|Transform|Lerp(Transform) (Variables|Default|GetA) (Variables|Default|GetB) _newtrack_0) false false))
          (:Finished
            (Default|EvShowDialogQuestAttack (CallFunction|BFLGetGameModeBP) (Variables|Default|GetBossOnLevel))))))))

(fn ConstructionScript)