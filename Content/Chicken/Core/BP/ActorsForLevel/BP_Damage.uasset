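; BP_Damage is a sprite-based level hazard that applies point damage to any actor that begins overlapping its PaperSprite.
; On BeginPlay, a timeline moves the sprite along its relative Z axis between a lowered position and its origin, without sweeping.
; The overlap event passes the Damage variable to ApplyPointDamage, using the hazard's location for the hit and itself as the damage causer.
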(event OnComponentBeginOverlap(PaperSprite)
  (params (OverlappedComponent :type Primitive%20Component%20Object%20Reference) (OtherActor :type Actor%20Object%20Reference) (OtherComp :type Primitive%20Component%20Object%20Reference) (OtherBodyIndex :type Integer) (bFromSweep :type Boolean) (SweepResult :type Hit%20Result%20Structure%20%28by%20ref%29))
  (bind _returnvalue (Transformation|GetActorLocation))
  (Game|Damage|ApplyPointDamage OtherActor (Variables|Default|GetDamage) _returnvalue (Collision|MakeHitResult false false 0.0 0.0 _returnvalue "0, 0, 0" "0,0,1" "0,0,1" 0 self) 0 self))

(event EventBeginPlay
  (bind _newtrack_0 (Timeline|Timeline_0 Play)
    (:Update
      (Transformation|SetRelativeLocation (Variables|Default|GetPaperSprite) (Math|Vector|Lerp(Vector) "0, 0,-75.000000" "0, 0, 0" _newtrack_0) false false))))

(fn ConstructionScript)